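; Shared helper functions for gameplay lookups and common actor operations on characters, items, skills and interactives.
; DataTable getters resolve row handles or enum-named rows into items, skills, materials, characters, NPCs, collectibles, rarity colors and attribute bonuses.
; Self-character checks use player controller 0, highlights use mesh custom depth, and hero clickability toggles the capsule's Visibility response.
; Movement helpers compute facing and make swept position nudges that report hit characters.
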(fn `Get Attribute Bonuses From Datatable`
  (params (Attribute :type "/Game/Blueprints/Characters/ScaleAttributes Enum" :default "NewEnumerator0"))
  (returns (`Attribute Bonuses` :type "/Game/Blueprints/Characters/AttributeBonuses Structure"))
  (bind _returnvalue (`|GetDataTableRow` "/Game/Blueprints/Characters/AttributeBonusesDatatable.AttributeBonusesDatatable" (`KismetStringLibrary.Conv_StringToName` (`|GetEnumeratorNameAsString` Attribute)))
    (:`then`
      (return _returnvalue))))

(fn `Get Character Forward Vector Towards Location`
  (params (Character :type "/Game/Blueprints/Characters/ABaseCharacter Object Reference") (Location :type "Vector Structure"))
  (returns (`Forward Vector` :type "Vector Structure"))
  (return (`KismetMathLibrary.GetForwardVector` (`KismetMathLibrary.FindLookAtRotation` (`Actor.K2_GetActorLocation` Character) (`local.Location`)))))

(fn `Get Character From Datatable`
  (params (`Datatable Row` :type "DataTableRowHandle Structure"))
  (returns (`Character Metadata` :type "/Game/Blueprints/Characters/CharacterMetadata Structure"))
  (bind (_datatable _rowname) (break `DataTableRowHandle` `Datatable Row`))
  (bind _returnvalue (`|GetDataTableRow` _datatable _rowname)
    (:`then`
      (return _returnvalue))))

(fn `Get Character Rotation Towards Direction`
  (params (Character :type "/Game/Blueprints/Characters/ABaseCharacter Object Reference") (Direction :type "Vector Structure"))
  (returns (Rotation :type "Rotator Structure"))
  (return (`KismetMathLibrary.MakeRotator` (.roll (`KismetMathLibrary.FindLookAtRotation` (`Actor.K2_GetActorLocation` Character) (`local.Direction`))) 0.0 (.yaw (`KismetMathLibrary.FindLookAtRotation` (`Actor.K2_GetActorLocation` Character) (`local.Direction`))))))

(fn `Get Collectible In Datatable`
  (params (`Datatable Entry` :type "DataTableRowHandle Structure"))
  (returns (Collectible :type "/Game/Blueprints/Interactives/Collectibles/Collectible Structure"))
  (bind (_datatable _rowname) (break `DataTableRowHandle` `Datatable Entry`))
  (bind _returnvalue (`|GetDataTableRow` _datatable _rowname)
    (:`then`
      (return _returnvalue))))

(fn `Get Item By Class Reference`
  (params (Items :type "Array of /Game/Blueprints/HUD/Bag/StatefulItemStructure Structure") (`Item Class Reference` :type "/Game/Blueprints/Interactives/Items/Item Class Reference"))
  (returns (`Success?` :type Boolean) (Index :type Integer) (`Item With State` :type "/Game/Blueprints/HUD/Bag/StatefulItemStructure Structure"))
  (locals (`Local Item With State` :type "/Game/Blueprints/HUD/Bag/StatefulItemStructure Structure") (`Local Index` :type Integer) (`Local Success?` :type Boolean))
  (for (_array_element _array_index) Items
    (if (== (`.ClassReference_36_3FAD921844AF363EE8BE1A8FA2AF7AFD` (break `/Game/Blueprints/Interactives/Items/Item_Info_Structure` (`.ItemInformation_11_1DD2AE774F3031A8B70F96BD9FF43819` (break `/Game/Blueprints/HUD/Bag/StatefulItemStructure` _array_element)))) (`local.Item Class Reference`))
      (set `local.Local Item With State` _array_element)
      (set `local.Local Index` _array_index)
      (set `local.Local Success?` true)
      (break)))
  (return (`local.Local Success?`) (`local.Local Index`) (`local.Local Item With State`)))

(fn `Get Item Information From Datatable`
  (params (`Item In Datatable` :type "DataTableRowHandle Structure"))
  (returns (`Success?` :type Boolean) (`Item Information` :type "/Game/Blueprints/Interactives/Items/Item_Info_Structure Structure"))
  (locals (`Local Item Information` :type "/Game/Blueprints/Interactives/Items/Item_Info_Structure Structure"))
  (bind (_datatable _rowname) (break `DataTableRowHandle` `Item In Datatable`))
  (bind _returnvalue (`|GetDataTableRow` _datatable _rowname)
    (:`then`
      (bind _output_get (set `local.Local Item Information` _returnvalue))
      (return true _output_get))
    (:`RowNotFound`
      (return false))))

(fn `Get Item Rarity Color`
  (params (`Item Rarity` :type "/Game/Blueprints/Interactives/Items/Item_Rarity_Types Enum" :default "NewEnumerator0"))
  (returns (Color :type "LinearColor Structure"))
  (bind _returnvalue (`|GetDataTableRow` "/Game/Blueprints/Interactives/Items/ItemRarityDropChances.ItemRarityDropChances" (`KismetStringLibrary.Conv_StringToName` (`|GetEnumeratorNameAsString` `Item Rarity`)))
    (:`then`
      (return (`.Color_12_D609993B4AAB35DCD4253EB5A2BCDC01` (break `/Game/Blueprints/Interactives/Items/RarityLootChanceStructure` _returnvalue))))))

(fn `Get Material From Datatable`
  (params (`Material In Datatable` :type "DataTableRowHandle Structure"))
  (returns (Material :type "/Game/Blueprints/Interactives/Items/Item_Info_Structure Structure"))
  (bind (_datatable _rowname) (break `DataTableRowHandle` `Material In Datatable`))
  (bind _returnvalue (`|GetDataTableRow` _datatable _rowname)
    (:`then`
      (return _returnvalue))))

(fn `Get NPC From Datatable`
  (params (Row :type "DataTableRowHandle Structure"))
  (returns (`NPC Metadata` :type "/Game/Blueprints/Characters/NPCs/NPCMetadata Structure"))
  (bind (_datatable _rowname) (break `DataTableRowHandle` Row))
  (bind _returnvalue (`|GetDataTableRow` _datatable _rowname)
    (:`then`
      (return _returnvalue))))

(fn `Get Player Controller`
  (params (Object :type "Object Object Reference"))
  (returns (`Player Controller` :type "/Game/Blueprints/Core/PlayerControllerMaster Object Reference"))
  (bind _asplayer_controller_master (cast `/Game/Blueprints/Core/PlayerControllerMaster` Object))
  (return _asplayer_controller_master))

(fn `Get Self Character`
  (returns (Character :type "/Game/Blueprints/Characters/AHeroCharacter Object Reference"))
  (bind _asplayer_controller_master (cast `/Game/Blueprints/Core/PlayerControllerMaster` (`GameplayStatics.GetPlayerController` null)))
  (return (`/Game/Blueprints/Core/PlayerControllerMaster.ControlledCharacter` _asplayer_controller_master)))

(fn `Get Skill Information From Datatable`
  (params (`Skill In Datatable` :type "DataTableRowHandle Structure"))
  (returns (`Skill Information` :type "/Game/Blueprints/Characters/Skills/SkillMetadata Structure"))
  (bind (_datatable _rowname) (break `DataTableRowHandle` `Skill In Datatable`))
  (bind _returnvalue (`|GetDataTableRow` _datatable _rowname)
    (:`then`
      (return _returnvalue))))

(fn `Get Skill Metadata`
  (params (Skill :type "/Game/Blueprints/Characters/Skills/Skill Class Reference"))
  (returns (Metadata :type "/Game/Blueprints/Characters/Skills/SkillMetadata Structure"))
  (return (`self.Get Skill Information From Datatable` (defaults `Object` Skill))))

(fn `Is Actor Highlighted?`
  (params (Actor :type "Actor Object Reference"))
  (returns (`Return Value` :type Boolean))
  (bind _asabase_character (cast `/Game/Blueprints/Characters/ABaseCharacter` Actor)
    (:`then`
      (return (`PrimitiveComponent.bRenderCustomDepth` (`Character.Mesh` _asabase_character))))
    (:`CastFailed`
      (bind _asainteractive (cast `/Game/Blueprints/Interactives/AInteractive` (`local.Actor`))
        (:`then`
          (return (`PrimitiveComponent.bRenderCustomDepth` (`/Game/Blueprints/Interactives/AInteractive.Mesh` _asainteractive))))
        (:`CastFailed`
          (return false))))))

(fn `Is Item Valid?`
  (params (Item :type "/Game/Blueprints/Interactives/Items/Item_Info_Structure Structure"))
  (returns (Return :type Boolean))
  (if (`KismetSystemLibrary.IsValidClass` (`.ClassReference_36_3FAD921844AF363EE8BE1A8FA2AF7AFD` (break `/Game/Blueprints/Interactives/Items/Item_Info_Structure` Item)))
    (return true)
    (else
      (return false))))

(fn `Is Self Character?`
  (params (Actor :type "Actor Object Reference"))
  (returns (ReturnValue :type Boolean))
  (bind _asplayer_controller_master (cast `/Game/Blueprints/Core/PlayerControllerMaster` (`GameplayStatics.GetPlayerController` null)))
  (return (== (`/Game/Blueprints/Core/PlayerControllerMaster.ControlledCharacter` _asplayer_controller_master) (`local.Actor`))))

(fn `Look At Location`
  (params (Character :type "/Game/Blueprints/Characters/ABaseCharacter Object Reference") (Location :type "Vector Structure"))
  (`Actor.K2_SetActorRotation` Character (`KismetMathLibrary.MakeRotator` (.roll (`KismetMathLibrary.FindLookAtRotation` (`Actor.K2_GetActorLocation` Character) (`local.Location`))) 0.0 (.yaw (`KismetMathLibrary.FindLookAtRotation` (`Actor.K2_GetActorLocation` Character) (`local.Location`)))) false))

(fn `Move Character Towards Rotation`
  (params (Character :type "/Game/Blueprints/Characters/ABaseCharacter Object Reference") (Rotation :type "Rotator Structure") (Force :type "Float (double-precision)") (`Stop Movements On Hit?` :type Boolean))
  (returns (`Hit Character` :type "/Game/Blueprints/Characters/ABaseCharacter Object Reference") (`Has Hit Another Character?` :type Boolean))
  (locals (`Final Force` :type "Float (double-precision)"))
  (bind _final_force (`local.Final Force`))
  (if (> (`local.Force`) 0.0)
    (set `local.Final Force` (`local.Force`))
    (else
      (set `local.Final Force` 50.0)))
  (bind (_sweephitresult _returnvalue) (`Actor.K2_SetActorLocation` (`local.Character`) (+ (`Actor.K2_GetActorLocation` (`local.Character`)) (* (`KismetMathLibrary.GetForwardVector` (`local.Rotation`)) (`KismetMathLibrary.MakeVector` _final_force _final_force))) true false))
  (if _returnvalue
    (bind (_bblockinghit _binitialoverlap _time _distance _location _impactpoint _normal _impactnormal _physmat _hitactor) (`GameplayStatics.BreakHitResult` _sweephitresult))
    (if _bblockinghit
      (if (`local.Stop Movements On Hit?`)
        (`/Game/Blueprints/Characters/ABaseCharacter.Stop Movements` (`local.Character`)))
      (bind _asabase_character (cast `/Game/Blueprints/Characters/ABaseCharacter` _hitactor)
        (:`then`
          (return _asabase_character true))
        (:`CastFailed`
          (return null false))))))

(fn `Remove Highlight From Actor`
  (params (Actor :type "Actor Object Reference"))
  (bind _asabase_character (cast `/Game/Blueprints/Characters/ABaseCharacter` Actor)
    (:`then`
      (`PrimitiveComponent.SetRenderCustomDepth` (`Character.Mesh` _asabase_character) false))
    (:`CastFailed`
      (bind _asainteractive (cast `/Game/Blueprints/Interactives/AInteractive` (`local.Actor`)))
      (`PrimitiveComponent.SetRenderCustomDepth` (`/Game/Blueprints/Interactives/AInteractive.Mesh` _asainteractive) false))))

(fn `Toggle Actor Clickability`
  (params (Actor :type "Actor Object Reference") (`On?` :type Boolean))
  (locals (`New Collision Response` :type "ECollisionResponse Enum"))
  (if `On?`
    (set `local.New Collision Response` "ECR_Block")
    (else
      (set `local.New Collision Response` "ECR_Ignore")))
  (bind _asahero_character (cast `/Game/Blueprints/Characters/AHeroCharacter` (`local.Actor`)))
  (`PrimitiveComponent.SetCollisionResponseToChannel` (`Character.CapsuleComponent` _asahero_character) "ECC_Visibility" (`local.New Collision Response`)))