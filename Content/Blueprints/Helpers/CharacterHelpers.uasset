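; Helper functions for characters that compute a maximum range and decide whether two characters are allied.
; GetMaxRange scales the current physical attack range by a stepped multiplier that is larger for short ranges and smaller for long ones.
; AreCharactersAllied relies on actor ownership, returning true when the second character owns the first or both share an owner, without checking the reverse ownership.
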(fn `Are Characters Allied?`
  (params (`Character 1` :type "/Game/Blueprints/Characters/ABaseCharacter Object Reference") (`Character 2` :type "/Game/Blueprints/Characters/ABaseCharacter Object Reference"))
  (returns (`Return Value` :type Boolean))
  (if (== (`Actor.GetOwner` (`local.Character 1`)) (`local.Character 2`))
    (return true)
    (elif (== (`Actor.GetOwner` (`local.Character 1`)) (`Actor.GetOwner` (`local.Character 2`)))
      (return true)
      (else
        (return false)))))

(fn `Get Max Range`
  (params (Character :type "/Game/Blueprints/Characters/ABaseCharacter Object Reference"))
  (returns (`Max Range` :type "Float (double-precision)"))
  (locals (Multiplier :type "Float (double-precision)"))
  (bind _current_physical_attack_range (`/Game/Blueprints/Characters/ABaseCharacter.Get Current Physical Attack Range` Character))
  (if (<= _current_physical_attack_range 100.0)
    (set `local.Multiplier` 5.0)
    (elif (<= _current_physical_attack_range 200.0)
      (set `local.Multiplier` 4.0)
      (elif (<= _current_physical_attack_range 300.0)
        (set `local.Multiplier` 3.0)
        (elif (<= _current_physical_attack_range 1000.0)
          (set `local.Multiplier` 3.0)
          (else
            (set `local.Multiplier` 2.0))))))
  (return (* (`/Game/Blueprints/Characters/ABaseCharacter.Get Current Physical Attack Range` (`local.Character`)) (`local.Multiplier`))))