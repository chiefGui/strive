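; Loot helper function that rolls random drops from a list of loot entries.
; Each entry is rolled independently against its percent chance to drop, so several items or none can come from one call.
; It returns the won items along with a flag that says whether anything was looted.
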(fn `Get Random Drop`
  (params (`From Loot` :type "Array of /Game/Blueprints/Characters/NPCs/Library/Enemies/LootItemStructure Structure"))
  (returns (`Looted Items` :type "Array of /Game/Blueprints/Interactives/Items/Item_Pickup Class Reference") (`Has looted something?` :type Boolean))
  (locals (Items :type "Array of /Game/Blueprints/Interactives/Items/Item_Pickup Class Reference"))
  (bind _items (`local.Items`))
  (for _array_element `From Loot`
    (bind (_item _chancetodrop) (break `/Game/Blueprints/Characters/NPCs/Library/Enemies/LootItemStructure` _array_element))
    (if (>= _chancetodrop (`KismetMathLibrary.RandomFloatInRange` 0.0 100.0))
      (`KismetArrayLibrary.Array_Add` (`local.Items`) _item)))
  (return _items (> (`KismetArrayLibrary.Array_Length` _items) 0)))