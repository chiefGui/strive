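; Particle helper functions for spawning beam effects between two characters and removing particle effects from a character.
; The beam spawn creates an emitter from the given template and passes both characters as "Source Actor" and "Target Actor" instance parameters.
; Removal finds the first CharacterParticle component whose particle system matches the template, destroys both components and returns whether it found one.
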(fn `Destroy Particle From Character`
  (params (Character :type "/Game/Blueprints/Characters/ABaseCharacter Object Reference") (`Particle System Template` :type "ParticleSystem Object Reference"))
  (returns (`Success?` :type Boolean))
  (locals (`Local Success?` :type Boolean) (`Local Character Particle Component` :type "/Game/Blueprints/Characters/Components/CharacterParticle Object Reference"))
  (for _array_element (`Actor.K2_GetComponentsByClass` Character "/Game/Blueprints/Characters/Components/CharacterParticle.CharacterParticle_C")
    (bind _particle_system_component (`/Game/Blueprints/Characters/Components/CharacterParticle.Particle System Component` _array_element))
    (`/Engine/EditorBlueprintResources/StandardMacros.IsValid` _particle_system_component
      (:`Is Valid`
        (if (== (`ParticleSystemComponent.Template` _particle_system_component) (`local.Particle System Template`))
          (set `local.Local Success?` true)
          (set `local.Local Character Particle Component` _array_element)
          (break)))))
  (if (`local.Local Success?`)
    (`ActorComponent.K2_DestroyComponent` (`/Game/Blueprints/Characters/Components/CharacterParticle.Particle System Component` (`local.Local Character Particle Component`)))
    (`ActorComponent.K2_DestroyComponent` (`local.Local Character Particle Component`))
    (return true)
    (else
      (return false))))

(fn `Spawn Beam Particle Between Characters`
  (params (`Source Character` :type "/Game/Blueprints/Characters/ABaseCharacter Object Reference") (`Target Character` :type "/Game/Blueprints/Characters/ABaseCharacter Object Reference") (`Particle System Template` :type "ParticleSystem Object Reference"))
  (returns (`Particle System Component` :type "ParticleSystemComponent Object Reference"))
  (bind _returnvalue (`GameplayStatics.SpawnEmitterAtLocation` null `Particle System Template`))
  (set `ParticleSystemComponent.InstanceParameters` (`|MakeArray` (make `ParticleSysParam` :`Name` "Source Actor" :`ParamType` "PSPT_Actor" :`Actor` (`local.Source Character`)) (make `ParticleSysParam` :`Name` "Target Actor" :`ParamType` "PSPT_Actor" :`Actor` (`local.Target Character`))) _returnvalue)
  (return _returnvalue))