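; ANPCSpawn is a server-authoritative spawn point that spawns one enemy and watches the area it may move within.
; On BeginPlay it spawns the Enemy class at the MovementArea location with the Arrow's rotation, passing itself as the spawn reference.
; MovementArea overlaps notify that enemy when other characters enter or leave, or when the enemy itself leaves.
; A RemoveEnemyFromSpawn event clears the reference, with no respawn here.
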(event `self.ReceiveBeginPlay`
  (`/Engine/EditorBlueprintResources/ActorMacros.Switch Has Authority`
    (:`Authority`
      (`self.Spawn`))))

(event `self.MovementArea.OnComponentBeginOverlap`
  (params (OverlappedComponent :type "PrimitiveComponent Object Reference") (OtherActor :type "Actor Object Reference") (OtherComp :type "PrimitiveComponent Object Reference") (OtherBodyIndex :type Integer) (bFromSweep :type Boolean) (SweepResult :type "HitResult Structure (by ref)"))
  (bind _spawned_enemy (`self.Spawned Enemy`))
  (`/Engine/EditorBlueprintResources/ActorMacros.Switch Has Authority`
    (:`Authority`
      (`/Engine/EditorBlueprintResources/StandardMacros.IsValid` (`self.Spawned Enemy`)
        (:`Is Valid`
          (bind _asabase_character (cast `/Game/Blueprints/Characters/ABaseCharacter` OtherActor))
          (if (!= _spawned_enemy _asabase_character)
            (`/Game/Blueprints/Characters/NPCs/ANPCCharacter.On Other Character Enters Movement Area (Server)` _spawned_enemy _asabase_character)))))))

(event `Remove Enemy From Spawn (Server)`
  (set `self.Spawned Enemy` null))

(event `self.MovementArea.OnComponentEndOverlap`
  (params (OverlappedComponent :type "PrimitiveComponent Object Reference") (OtherActor :type "Actor Object Reference") (OtherComp :type "PrimitiveComponent Object Reference") (OtherBodyIndex :type Integer))
  (`/Engine/EditorBlueprintResources/ActorMacros.Switch Has Authority`
    (:`Authority`
      (`/Engine/EditorBlueprintResources/StandardMacros.IsValid` (`self.Spawned Enemy`)
        (:`Is Valid`
          (if (== (`self.Spawned Enemy`) OtherActor)
            (`/Game/Blueprints/Characters/NPCs/ANPCCharacter.On Leave Movement Area (Server)` (`self.Spawned Enemy`))
            (else
              (bind _asabase_character (cast `/Game/Blueprints/Characters/ABaseCharacter` OtherActor))
              (`/Engine/EditorBlueprintResources/StandardMacros.IsValid` _asabase_character
                (:`Is Valid`
                  (`/Game/Blueprints/Characters/NPCs/ANPCCharacter.On Other Character Leaves Movement Area (Server)` (`self.Spawned Enemy`) _asabase_character))))))))))

(fn `Spawn`
  (bind _returnvalue (`|SpawnActorFromClass` (`self.Enemy`) (`KismetMathLibrary.MakeTransform` (`SceneComponent.K2_GetComponentLocation` (`self.MovementArea`)) (`SceneComponent.K2_GetComponentRotation` (`self.Arrow`))) "AlwaysSpawn" "OverrideRootScale" null self null))
  (set `self.Spawned Enemy` _returnvalue))

(fn `UserConstructionScript`)