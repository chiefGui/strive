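; ASpawn is a one-shot random spawn point that, on BeginPlay with authority, picks an actor class from Possibilities and spawns it at its root location.
; With IgnoreChances it picks any entry at random.
; Otherwise one 0-100 roll selects the first entry whose Chance meets it, so array order matters and chances are not summed.
; It destroys itself after spawning, but remains if no valid class is chosen.
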(event `self.ReceiveBeginPlay`
  (`/Engine/EditorBlueprintResources/ActorMacros.Switch Has Authority`
    (:`Authority`
      (if (`self.Ignore Chances?`)
        (bind _element (`/Game/Blueprints/Helpers/LodashMacros.Get Random Element From Array` (`self.Possibilities`))
          (:`Done`
            (`self.Spawn Actor` (`.Actor_7_2D010660418AFAA8279D58988537FFD1` (break `/Game/Blueprints/Spawns/SpawnStructure` _element)))))
        (else
          (bind (_success_ _chosen_actor) (`self.Get Random Actor To Spawn`))
          (if _success_
            (`self.Spawn Actor` _chosen_actor)))))))

(fn `Get Random Actor To Spawn`
  (returns (`Success?` :type Boolean) (`Chosen Actor` :type "Actor Class Reference"))
  (locals (`Local Chosen Actor` :type "Actor Class Reference") (`Dice Result` :type "Float (double-precision)"))
  (bind _local_chosen_actor (`local.Local Chosen Actor`))
  (set `local.Dice Result` (`KismetMathLibrary.RandomFloatInRange` 0.0 100.0))
  (for _array_element (`self.Possibilities`)
    (bind (_actor _chance) (break `/Game/Blueprints/Spawns/SpawnStructure` _array_element))
    (if (>= _chance (`local.Dice Result`))
      (set `local.Local Chosen Actor` _actor)
      (break)))
  (if (`KismetSystemLibrary.IsValidClass` _local_chosen_actor)
    (return true _local_chosen_actor)
    (else
      (return false null))))

(fn `Spawn Actor`
  (params (Actor :type "Actor Class Reference"))
  (`|SpawnActorFromClass` Actor (`KismetMathLibrary.MakeTransform` (`SceneComponent.K2_GetComponentLocation` (`self.DefaultSceneRoot`))) "Undefined" "OverrideRootScale" null null)
  (`self.K2_DestroyActor`))

(fn `UserConstructionScript`)