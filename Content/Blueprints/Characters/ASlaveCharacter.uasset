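; Character Blueprint for an allied "slave" NPC bound to a master character, which the server takes from the actor's owner at construction.
; The server kills it after an optional lifetime, while allied clients swap its standard NPC widget for a quick-data widget.
; Attribute refreshes push HP to the master's controller, and death calls the ally destruction routine and multicasts widget removal to clients.
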(event `self.ReceiveBeginPlay`
  (bind _returnvalue (`GameplayStatics.GetPlayerController` 0))
  (`parent.ReceiveBeginPlay`)
  (`/Engine/EditorBlueprintResources/ActorMacros.Switch Has Authority`
    (:`Authority`
      (if (> (`self.Life Duration`) 0.0)
        (`KismetSystemLibrary.Delay` (`self.Life Duration`))
        (`self.Self Suicide (Server)`)))
    (:`Remote`
      (bind _asplayer_controller_master (cast `/Game/Blueprints/Core/PlayerControllerMaster` _returnvalue))
      (bind _controlledcharacter (`/Game/Blueprints/Core/PlayerControllerMaster.ControlledCharacter` _asplayer_controller_master))
      (`/Engine/EditorBlueprintResources/StandardMacros.IsValid` _controlledcharacter
        (:`Is Valid`
          (if (`/Game/Blueprints/Characters/CharacterHelpers.Are Characters Allied?` _controlledcharacter self)
            (`ActorComponent.K2_DestroyComponent` (`self.NPCQuickDataWidget`))
            (bind _returnvalue_2 (`|CreateWidget` "/Game/Blueprints/HUD/NPCs/NPCQuickData.NPCQuickData_C" _returnvalue))
            (`WidgetComponent.SetWidget` (`self.SlaveQuickDataWidget`) _returnvalue_2)
            (set `/Game/Blueprints/HUD/NPCs/NPCQuickData.NPC` self _returnvalue_2)
            (set `self.SlaveQuickDataWidgetInstance` _returnvalue_2)))))))

(event `self.Kill`
  (`parent.Kill`)
  (`self.Destroy Ally (Server)` self)
  (`self.Remove Quick Data (Multicast)`))

(event `/Game/Blueprints/Characters/ICharacter.On Refresh Attributes`
  (params (`Displayable Attributes` :type "/Game/Blueprints/Characters/CharacterDisplayableAttributes Structure"))
  (`parent.On Refresh Attributes` `Displayable Attributes`)
  (bind _asplayer_controller_master (cast `/Game/Blueprints/Core/PlayerControllerMaster` (`self.GetOwner` (`self.Master Character`))))
  (`/Game/Blueprints/Core/PlayerControllerMaster.Update Ally HP (Own Client)` _asplayer_controller_master self (`self.Get Current HP` self) (`.Current` (`self.Get Max HP` self))))

(event `Remove Quick Data (Multicast)`
  (`/Engine/EditorBlueprintResources/ActorMacros.Switch Has Authority`
    (:`Remote`
      (`ActorComponent.K2_DestroyComponent` (`self.SlaveQuickDataWidget`)))))

(fn `UserConstructionScript`
  (`parent.UserConstructionScript`)
  (`/Engine/EditorBlueprintResources/ActorMacros.Switch Has Authority`
    (:`Authority`
      (bind _asabase_character (cast `/Game/Blueprints/Characters/ABaseCharacter` (`self.GetOwner`)))
      (set `self.Master Character` _asabase_character))))