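; Server-driven base NPC character that roams and fights inside the movement area of its spawn.
; Chasers target sensed hostile characters within that area, and being attacked or provoked also sets the target, which aggressive NPCs pursue and attack.
; Leaving the area drops the target, sends the NPC back and regenerates its health.
; Death deregisters it from the spawn, with optional delayed respawn, and a helper spawns chance-rolled loot chests.
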(event `/Game/Blueprints/Characters/ICharacter.While Target Is Valid (Server)`
  (if (`self.Is Aggressive Against Current Target?`)
    (if (`self.Is Current Target Within Attack Range?`)
      (`self.Attack Current Target`)
      (`self.Look At Actor` (`self.Current Target`))
      (else
        (`self.Move Towards Current Target`)))))

(event `/Game/Blueprints/Characters/ICharacter.On Idle (Server)`
  (if (`self.Is Roamer?`)
    (if (not (`self.Is Resting?`))
      (`self.Move to Destination Within Movement Area`))))

(event `/Game/Blueprints/Characters/ICharacter.On Reached Destination (Server)`
  (set `self.Is Resting?` true)
  (`KismetSystemLibrary.Delay` (`self.Rest Duration`))
  (set `self.Is Resting?` false))

(event `On Leave Movement Area (Server)`
  (if (not (`self.Is Dead?`))
    (set `self.Current Target` null)
    (`self.Move to Destination Within Movement Area`)
    (`/Game/Blueprints/Helpers/Time_Macros.Repeater` 2.0 :!label _label
      (:`On Every Interval`
        (if (`self.Is Dead?`)
          (goto _label :!via `Stop`)
          (else
            (bind _new_current_hp (`self.Increase Current HP` (`KismetMathLibrary.Conv_IntToDouble` (/ (`self.Get Current Max HP`) 2))))
            (if (>= _new_current_hp (`self.Get Current Max HP`))
              (goto _label :!via `Stop`))))))))

(event `self.ReceiveBeginPlay`
  (`parent.ReceiveBeginPlay`)
  (`/Engine/EditorBlueprintResources/ActorMacros.Switch Has Authority`))

(event `Provoke (Server)`
  (params (`Provoker Character` :type "/Game/Blueprints/Characters/ABaseCharacter Object Reference"))
  (set `self.Current Target` `Provoker Character`))

(event `/Game/Blueprints/Characters/ICharacter.On Attacked (Server)`
  (params (Attacker :type "/Game/Blueprints/Characters/ABaseCharacter Object Reference"))
  (set `self.Current Target` Attacker))

(event `On Other Character Enters Movement Area (Server)`
  (params (`Other Character` :type "/Game/Blueprints/Characters/ABaseCharacter Object Reference"))
  (`KismetArrayLibrary.Array_Add` (`self.Characters Within Movement Area`) `Other Character`))

(event `On Other Character Leaves Movement Area (Server)`
  (params (`Other Character` :type "/Game/Blueprints/Characters/ABaseCharacter Object Reference"))
  (`KismetArrayLibrary.Array_RemoveItem` (`self.Characters Within Movement Area`) `Other Character`))

(event `/Game/Blueprints/Characters/ICharacter.On Death (Server)`
  (params (`Killer Character` :type "/Game/Blueprints/Characters/ABaseCharacter Object Reference"))
  (`/Game/Blueprints/Spawns/AEnemySpawn.Remove Enemy From Spawn (Server)` (`self.Spawn`)))

(event `/Game/Blueprints/Characters/ICharacter.After Death Animation (Server)`
  (`KismetSystemLibrary.Delay` 2.0)
  (if (`self.Does Respawn?`)
    (`SceneComponent.SetVisibility` (`self.Mesh`) false false)
    (`KismetSystemLibrary.Delay` (`self.Respawn Time`))
    (`/Game/Blueprints/Spawns/AEnemySpawn.Spawn` (`self.Spawn`))
    (`self.K2_DestroyActor`)
    (else
      (`self.K2_DestroyActor`))))

(event `self.PawnSensing.OnSeePawn`
  (params (Pawn :type "Pawn Object Reference"))
  (`/Engine/EditorBlueprintResources/ActorMacros.Switch Has Authority`
    (:`Authority`
      (`self.Resolve Pawn Sensing (Server)` Pawn))))

(fn `Drop Chest Loot`
  (if (> (`KismetArrayLibrary.Array_Length` (`self.Potential Loot`)) 0)
    (bind _output_get (set `self.Actual Loot` (`self.Get Random Loot`)))
    (if (> (`KismetArrayLibrary.Array_Length` _output_get) 0)
      (`|SpawnActorFromClass` "/Game/Blueprints/Interactives/Chests/ACharacterChest.ACharacterChest_C" (`KismetMathLibrary.MakeTransform` (`SceneComponent.K2_GetComponentLocation` (`self.Mesh`))) "AlwaysSpawn" "OverrideRootScale" null _output_get null))))

(fn `Get Random Location Within Movement Area`
  (returns (Location :type "Vector Structure"))
  (bind _movementarea (`/Game/Blueprints/Spawns/AEnemySpawn.MovementArea` (`self.Spawn`)))
  (return (`NavigationSystem.K2_GetRandomLocationInNavigableRadius` (`SceneComponent.K2_GetComponentLocation` _movementarea) (`SphereComponent.SphereRadius` _movementarea))))

(fn `Get Random Loot`
  (returns (Loot :type "Array of /Game/Blueprints/HUD/Bag/StatefulItemStructure Structure"))
  (locals (`Items To Loot` :type "Array of /Game/Blueprints/HUD/Bag/StatefulItemStructure Structure"))
  (`/Engine/EditorBlueprintResources/ActorMacros.Switch Has Authority`
    (:`Authority`
      (for _array_element (`self.Potential Loot`)
        (if (>= (`.Chancetodrop_7_EF56E0FD40A48DCC927F17B6D7724CCA` (break `/Game/Blueprints/Characters/Library/NPCs/LootItemStructure` _array_element)) (`KismetMathLibrary.RandomFloatInRange` 0.0 100.0))
          (`KismetArrayLibrary.Array_Add` (`local.Items To Loot`) (make `/Game/Blueprints/HUD/Bag/StatefulItemStructure` (`.Item Information` (`/Game/Blueprints/Helpers/Helpers.Get Item Information From Datatable` (defaults `/Game/Blueprints/Characters/ANPCCharacter` (break `/Game/Blueprints/Characters/Library/NPCs/LootItemStructure` _array_element)))) 1))))
      (return (`local.Items To Loot`)))))

(fn `Is Character Within Movement Area?`
  (params (Character :type "/Game/Blueprints/Characters/ABaseCharacter Object Reference"))
  (returns (`Return Value` :type Boolean))
  (locals (`Local Bool` :type Boolean))
  (for _array_element (`self.Characters Within Movement Area`)
    (if (== _array_element (`local.Character`))
      (set `local.Local Bool` true)
      (break)))
  (return (`local.Local Bool`)))

(fn `Move to Destination Within Movement Area`
  (`self.Move To Destination (Server)` (`self.Get Random Location Within Movement Area`)))

(fn `Resolve Pawn Sensing (Server)`
  (params (Pawn :type "Pawn Object Reference"))
  (locals (`Seen Character` :type "/Game/Blueprints/Characters/ABaseCharacter Object Reference"))
  (if (not (`self.Is Dead?`))
    (bind _asabase_character (cast `/Game/Blueprints/Characters/ABaseCharacter` (`local.Pawn`)))
    (bind _output_get (set `local.Seen Character` _asabase_character))
    (if (`/Game/Blueprints/Characters/ABaseCharacter.Is Dead?` _output_get)
      _
      (elif (`self.Is Character Within Movement Area?` (`local.Seen Character`))
        (if (`self.Is Chaser?`)
          (if (`self.Is Aggressive Against Actor?` (`local.Seen Character`))
            (if (not (`self.Is Attacking?`))
              (set `self.Current Target` (`local.Seen Character`)))))))))

(fn `UserConstructionScript`
  (`parent.UserConstructionScript`))