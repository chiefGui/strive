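; Server-side manager that adds and removes stat modifiers on its owning ABaseCharacter, which it caches on BeginPlay with authority.
; AddModifier maps a stat type to the character's matching Add function and returns the created modifier.
; Batch adds and item removals suppress per-modifier client updates, then request one attribute refresh.
; "Gracefully" variants apply non-stacking item effects only for the first equipped copy and remove them with the last.
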(event `self.ReceiveBeginPlay`
  (`/Engine/EditorBlueprintResources/ActorMacros.Switch Has Authority`
    (:`Authority`
      (bind _asabase_character (cast `/Game/Blueprints/Characters/ABaseCharacter` (`self.GetOwner`)))
      (set `self.Character` _asabase_character))))

(fn `Add Item Modifiers`
  (params (Item :type "/Game/Blueprints/Interactives/Items/ItemStructure Structure"))
  (bind ((`Name_2_359C4861424747F5E3870B984A1ED0E6` _name) (`Modifiers_93_F2D4811D47C206977D423690262A915F` _modifiers)) (break `/Game/Blueprints/Interactives/Items/ItemStructure` Item))
  (`self.Add Modifiers` _name _modifiers))

(fn `Add Item Modifiers Gracefully`
  (params (Item :type "/Game/Blueprints/Interactives/Items/ItemStructure Structure") (`Equipped Items` :type "Array of /Game/Blueprints/Interactives/Items/ItemStructure Structure"))
  (if (`.DoesEffectStack?_73_48CF15384B2CE29BB9CDFD919B8AD2BD` (break `/Game/Blueprints/Interactives/Items/ItemStructure` Item))
    (`self.Add Item Modifiers` (`local.Item`))
    (elif (`/Game/Helpers/ItemsHelpers.Is First Item In Items?` (`local.Item`) (`local.Equipped Items`))
      (`self.Add Item Modifiers` (`local.Item`)))))

(fn `Add Modifier`
  (params (`Modifier Component` :type "/Game/Blueprints/Characters/Modifiers Enum" :default "NewEnumerator0") (Amount :type "Float (double-precision)") (Duration :type "Float (double-precision)") (ID :type Name) (`Automatically Dispatch An Update To Client?` :type Boolean :default true))
  (returns (Modifier :type "/Game/Blueprints/Characters/Modifiers/CModifier Object Reference"))
  (locals (`Local Modifier Component` :type "/Game/Blueprints/Characters/Modifiers/CModifier Object Reference") (`Local Duration` :type "Float (double-precision)"))
  (set `local.Local Duration` Duration)
  (switch `/Game/Blueprints/Characters/Modifiers` `Modifier Component`
    (:`NewEnumerator0`
      (bind _returnvalue (`AddComponent|NODE_AddCHPModifier-0` :`self` (`self.Character`) :`Amount` (`KismetMathLibrary.FTrunc` (`local.Amount`)) :`ID` (`local.ID`) :`Duration` (`local.Local Duration`) :`Automatically Dispatch Client Update?` (`local.Automatically Dispatch An Update To Client?`)))
      (set `local.Local Modifier Component` _returnvalue))
    (:`NewEnumerator1`
      (bind _returnvalue_2 (`AddComponent|NODE_AddCMPModifier-0` :`self` (`self.Character`) :`Amount` (`KismetMathLibrary.FTrunc` (`local.Amount`)) :`ID` (`local.ID`) :`Duration` (`local.Local Duration`) :`Automatically Dispatch Client Update?` (`local.Automatically Dispatch An Update To Client?`)))
      (set `local.Local Modifier Component` _returnvalue_2))
    (:`NewEnumerator2`
      (bind _returnvalue_3 (`AddComponent|NODE_AddCHPRegenModifier-0` :`self` (`self.Character`) :`Amount` (`local.Amount`) :`ID` (`local.ID`) :`Duration` (`local.Local Duration`) :`Automatically Dispatch Client Update?` (`local.Automatically Dispatch An Update To Client?`)))
      (set `local.Local Modifier Component` _returnvalue_3))
    (:`NewEnumerator3`
      (bind _returnvalue_4 (`AddComponent|NODE_AddCMPRegenModifier-0` :`self` (`self.Character`) :`Amount` (`local.Amount`) :`ID` (`local.ID`) :`Duration` (`local.Local Duration`) :`Automatically Dispatch Client Update?` (`local.Automatically Dispatch An Update To Client?`)))
      (set `local.Local Modifier Component` _returnvalue_4))
    (:`NewEnumerator4`
      (bind _returnvalue_5 (`AddComponent|NODE_AddCPhysicalDamageModifier-0` :`self` (`self.Character`) :`Amount` (`local.Amount`) :`ID` (`local.ID`) :`Duration` (`local.Local Duration`) :`Automatically Dispatch Client Update?` (`local.Automatically Dispatch An Update To Client?`)))
      (set `local.Local Modifier Component` _returnvalue_5))
    (:`NewEnumerator5`
      (bind _returnvalue_6 (`AddComponent|NODE_AddCPhysicalDefenseModifier-0` :`self` (`self.Character`) :`Amount` (`local.Amount`) :`ID` (`local.ID`) :`Duration` (`local.Local Duration`) :`Automatically Dispatch Client Update?` (`local.Automatically Dispatch An Update To Client?`)))
      (set `local.Local Modifier Component` _returnvalue_6))
    (:`NewEnumerator15`
      (bind _returnvalue_7 (`AddComponent|NODE_AddMagicalDamageModifier-0` :`self` (`self.Character`) :`Amount` (`local.Amount`) :`ID` (`local.ID`) :`Duration` (`local.Local Duration`) :`Automatically Dispatch Client Update?` (`local.Automatically Dispatch An Update To Client?`)))
      (set `local.Local Modifier Component` _returnvalue_7))
    (:`NewEnumerator16`
      (bind _returnvalue_8 (`AddComponent|NODE_AddMagicalDefenseModifier-0` :`self` (`self.Character`) :`Amount` (`local.Amount`) :`ID` (`local.ID`) :`Duration` (`local.Local Duration`) :`Automatically Dispatch Client Update?` (`local.Automatically Dispatch An Update To Client?`)))
      (set `local.Local Modifier Component` _returnvalue_8))
    (:`NewEnumerator8`
      (bind _returnvalue_9 (`AddComponent|NODE_AddCNeutralPhysicalDamageModifier-0` :`self` (`self.Character`) :`Amount` (`local.Amount`) :`ID` (`local.ID`) :`Duration` (`local.Local Duration`) :`Automatically Dispatch Client Update?` (`local.Automatically Dispatch An Update To Client?`)))
      (set `local.Local Modifier Component` _returnvalue_9))
    (:`NewEnumerator6`
      (bind _returnvalue_10 (`AddComponent|NODE_AddCASPDModifier-0` :`self` (`self.Character`) :`Amount` (`local.Amount`) :`ID` (`local.ID`) :`Duration` (`local.Local Duration`) :`Automatically Dispatch Client Update?` (`local.Automatically Dispatch An Update To Client?`)))
      (set `local.Local Modifier Component` _returnvalue_10))
    (:`NewEnumerator7`
      (bind _returnvalue_11 (`AddComponent|NODE_AddCWalkSpeedModifier-0` :`self` (`self.Character`) :`Amount` (`local.Amount`) :`ID` (`local.ID`) :`Duration` (`local.Local Duration`) :`Automatically Dispatch Client Update?` (`local.Automatically Dispatch An Update To Client?`)))
      (set `local.Local Modifier Component` _returnvalue_11))
    (:`NewEnumerator10`
      (bind _returnvalue_12 (`AddComponent|NODE_AddCStrengthModifier-0` :`self` (`self.Character`) :`Amount` (`local.Amount`) :`ID` (`local.ID`) :`Duration` (`local.Local Duration`) :`Automatically Dispatch Client Update?` (`local.Automatically Dispatch An Update To Client?`)))
      (set `local.Local Modifier Component` _returnvalue_12))
    (:`NewEnumerator11`
      (bind _returnvalue_13 (`AddComponent|NODE_AddCAgilityModifier-0` :`self` (`self.Character`) :`Amount` (`local.Amount`) :`ID` (`local.ID`) :`Duration` (`local.Local Duration`) :`Automatically Dispatch Client Update?` (`local.Automatically Dispatch An Update To Client?`)))
      (set `local.Local Modifier Component` _returnvalue_13))
    (:`NewEnumerator12`
      (bind _returnvalue_14 (`AddComponent|NODE_AddCIntelligenceModifier-0` :`self` (`self.Character`) :`Amount` (`local.Amount`) :`ID` (`local.ID`) :`Duration` (`local.Local Duration`) :`Automatically Dispatch Client Update?` (`local.Automatically Dispatch An Update To Client?`)))
      (set `local.Local Modifier Component` _returnvalue_14))
    (:`NewEnumerator13`
      (bind _returnvalue_15 (`AddComponent|NODE_AddCVitalityModifier-0` :`self` (`self.Character`) :`Amount` (`local.Amount`) :`ID` (`local.ID`) :`Duration` (`local.Local Duration`) :`Automatically Dispatch Client Update?` (`local.Automatically Dispatch An Update To Client?`)))
      (set `local.Local Modifier Component` _returnvalue_15)))
  (return (`local.Local Modifier Component`)))

(fn `Add Modifiers`
  (params (ID :type Name) (Modifiers :type "Array of /Game/Modifiers/Modifier Structure"))
  (for _array_element Modifiers
    (`self.Add Modifier` (`.Modifier_2_491C26B94205AA3DCF35ECB7EE619210` (break `/Game/Modifiers/Modifier` _array_element)) (`/Game/Helpers/ModifierHelpers.Get Final Modifier Amount` (`self.Character`) _array_element) 0.0 (`local.ID`) false))
  (if (`/Game/Helpers/ModifierHelpers.Has Any Modifier?` (`local.Modifiers`))
    (`/Game/Blueprints/Characters/ABaseCharacter.Request Refresh Attributes` (`self.Character`))))

(fn `Destroy Modifier`
  (params (Modifier :type "/Game/Blueprints/Characters/Modifiers/CModifier Object Reference") (`Dispatch Update To Client?` :type Boolean))
  (`/Game/Blueprints/Characters/Modifiers/CModifier.Full Destroy (Server)` Modifier `Dispatch Update To Client?`))

(fn `Remove Item Modifiers`
  (params (Item :type "/Game/Blueprints/Interactives/Items/ItemStructure Structure"))
  (locals (`Modifiers To Destroy` :type "Array of /Game/Blueprints/Characters/Modifiers/CModifier Object Reference") (`All Modifiers Of Item` :type "Array of /Game/Blueprints/Characters/Modifiers/CModifier Object Reference"))
  (set `local.All Modifiers Of Item` (`/Game/Helpers/ModifierHelpers.Get Modifiers Of Item In Character` (`self.Character`) (`local.Item`)))
  (for _array_element (`.Modifiers_93_F2D4811D47C206977D423690262A915F` (break `/Game/Blueprints/Interactives/Items/ItemStructure` (`local.Item`)))
    (for _array_element_2 (`local.All Modifiers Of Item`)
      (if (== (`GameplayStatics.GetObjectClass` _array_element_2) (`.ModifierClass_11_0AB97D6A426BAE26DD60C5A1A18F6FD5` (break `/Game/Modifiers/Modifier` _array_element)))
        (`KismetArrayLibrary.Array_Add` (`local.Modifiers To Destroy`) _array_element_2)
        (break))))
  (bind (_arrayindex _arrayelement) (`/Engine/EditorBlueprintResources/StandardMacros.ReverseForEachLoop` (`local.Modifiers To Destroy`))
    (:`LoopBody`
      (`self.Destroy Modifier` _arrayelement))
    (:`Completed`
      (`/Game/Blueprints/Characters/ABaseCharacter.Request Refresh Attributes` (`self.Character`)))))

(fn `Remove Item Modifiers Gracefully`
  (params (Item :type "/Game/Blueprints/Interactives/Items/ItemStructure Structure") (`Equipped Items` :type "Array of /Game/Blueprints/Interactives/Items/ItemStructure Structure"))
  (if (`.DoesEffectStack?_73_48CF15384B2CE29BB9CDFD919B8AD2BD` (break `/Game/Blueprints/Interactives/Items/ItemStructure` Item))
    (`self.Remove Item Modifiers` (`local.Item`))
    (elif (`/Game/Helpers/ItemsHelpers.Is Last Item In Items?` (`local.Item`) (`local.Equipped Items`))
      (`self.Remove Item Modifiers` (`local.Item`)))))

(fn `UserConstructionScript`)