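; Player-controlled hero character that relays gameplay events (combat, skills, XP, attributes, bushes, target HP) to its PlayerController for HUD and state updates.
; The server walks it to interactive targets and interacts when in range.
; Collecting runs as a server component with a client progress widget, stops on movement, and awards loot materials, as do NPC kills.
; Death drops items in a chest and transfers materials to a killing hero.
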(event `/Game/Blueprints/Characters/ICharacter.On Load (From Server)`)

(event `/Game/Blueprints/Characters/ICharacter.On Load (From Client)`
  (bind _player_controller (`/Game/Blueprints/Helpers/Helpers.Get Player Controller` (`self.GetOwner`)))
  (`/Engine/EditorBlueprintResources/StandardMacros.IsValid` _player_controller
    (:`Is Valid`
      (`/Game/Blueprints/Core/PlayerControllerMaster.On Hero Ready (Own Client)` _player_controller self))))

(event `/Game/Blueprints/Characters/ICharacter.On Actor Enter Bush`
  (params (`Actor That Entered` :type "Actor Object Reference") (Bush :type "/Game/Blueprints/Level/ABush Object Reference"))
  (`/Game/Blueprints/Core/PlayerControllerMaster.On Enter Bush (Own Client)` (`self.Player Controller`) (`/Game/Blueprints/Level/ABush.Actors Inside` Bush)))

(event `/Game/Blueprints/Characters/ICharacter.On Actor Leave Bush`
  (params (`Actor That Left` :type "Actor Object Reference") (Bush :type "/Game/Blueprints/Level/ABush Object Reference"))
  (`/Game/Blueprints/Core/PlayerControllerMaster.On Leave Bush (Own Client)` (`self.Player Controller`) `Actor That Left` (`/Game/Blueprints/Level/ABush.Actors Inside` Bush)))

(event `self.On Move (Server)`
  ;[0 0.4422 1] On Move (server)
  (if (`.Return Value` (`self.Is Collecting?`))
    (`self.Stop Collecting (Multicast)`)))

(event `/Game/Blueprints/Characters/ICharacter.On Death`
  (params (`Killer Character` :type "/Game/Blueprints/Characters/ABaseCharacter Object Reference"))
  ;[1 1 1] On this character dies
  (`/Engine/EditorBlueprintResources/ActorMacros.Switch Has Authority`
    (:`Authority`
      (`/Game/Blueprints/Core/FFAGameState.On Player's Death (Server)` (`/Game/Blueprints/Core/PlayerControllerMaster.Game State` (`self.Player Controller`)) (`self.Player Controller`))
      (`self.Give Items To Other Character` `Killer Character`)
      (`/Game/Blueprints/Core/PlayerControllerMaster.On Death (Server)` (`self.Player Controller`))
      (`self.Stop Collecting (Multicast)`))))

(event `self.While Has Interactive Target (Server)`
  (params (Interactive :type "/Game/Blueprints/Interactives/AInteractive Object Reference"))
  ;[1 1 1] While Has Interactive Target
  (`/Engine/EditorBlueprintResources/StandardMacros.IsValid` Interactive
    (:`Is Valid`
      (if (`self.Is In Interaction Range?` Interactive)
        (`/Game/Blueprints/Interactives/AInteractive.Interact (Multicast)` Interactive (`self.Player Controller`))
        (`self.Stop Movements`)
        (`self.Look At Actor` (`.Target Actor` (`self.Get Target`)))
        (`self.Remove Target`)
        (elif (`self.Is Walking?`)
          (goto _label :!via `Reset`)
          (else
            (`/Engine/EditorBlueprintResources/StandardMacros.DoOnce` false :!label _label
              (:`Completed`
                (`self.Move Towards Current Target`)))))))))

(event `/Game/Blueprints/Characters/ICharacter.On XP is increased`
  (params (`New Current XP` :type Integer) (`Levels Increased` :type Integer))
  (bind (_current_level _xp_needed _next_level_xp) (`self.Get Current Level`))
  (`/Game/Blueprints/Core/PlayerControllerMaster.Update XP Widget (Own Client)` (`self.Player Controller`) `New Current XP` _xp_needed _next_level_xp)
  (if (> `Levels Increased` 0)
    (`/Game/Blueprints/Core/PlayerControllerMaster.On Level Increase (Server)` (`self.Player Controller`) `Levels Increased`)))

(event `Start Collecting`
  (params (Collectible :type "/Game/Blueprints/Interactives/Collectibles/ACollectible Object Reference"))
  (`/Engine/EditorBlueprintResources/ActorMacros.Switch Has Authority`
    (:`Authority`
      (`AddComponent|NODE_AddCollecting-0` :`Collectible` Collectible))
    (:`Remote`
      (`self.Start Cast Progress Widget` (`.CollectionTime_21_AFEAF1274DC81134C186BAA7F55E69C8` (break `/Game/Blueprints/Interactives/Collectibles/Collectible` (`/Game/Blueprints/Helpers/Helpers.Get Collectible In Datatable` (`/Game/Blueprints/Interactives/Collectibles/ACollectible.Datatable Entry` Collectible))))))))

(event `self.ReceiveBeginPlay`
  (`parent.ReceiveBeginPlay`)
  (bind _asplayer_controller_master (cast `/Game/Blueprints/Core/PlayerControllerMaster` (`self.GetOwner`)))
  (set `self.Player Controller` _asplayer_controller_master))

(event `self.Collecting Success (Server)`
  (params (`Collecting Component` :type "/Game/Blueprints/Characters/Components/Collecting Object Reference") (Collectible :type "/Game/Blueprints/Interactives/Collectibles/ACollectible Object Reference"))
  (if (not (`Actor.bHidden` Collectible))
    (`/Game/Blueprints/Core/PlayerControllerMaster.On Collect Materials (Server)` (`self.Player Controller`) (`.LootMaterials_23_81027F164CEA83A488F9A4A2F9320A1C` (break `/Game/Blueprints/Interactives/Collectibles/Collectible` (`/Game/Blueprints/Helpers/Helpers.Get Collectible In Datatable` (`/Game/Blueprints/Interactives/Collectibles/ACollectible.Datatable Entry` Collectible)))))
    (`ActorComponent.K2_DestroyComponent` `Collecting Component`)
    (`/Game/Blueprints/Interactives/Collectibles/ACollectible.On Collected (Server)` Collectible)))

(event `/Game/Blueprints/Characters/ICharacter.On Refresh Attributes`
  (params (`Displayable Attributes` :type "/Game/Blueprints/Characters/CharacterDisplayableAttributes Structure"))
  (bind _player_controller (`self.Player Controller`))
  (`/Engine/EditorBlueprintResources/StandardMacros.IsValid` _player_controller
    (:`Is Valid`
      (`/Game/Blueprints/Core/PlayerControllerMaster.Refresh Attributes On HUD (Own Client)` _player_controller `Displayable Attributes`))))

(event `/Game/Blueprints/Characters/ICharacter.On Target Lost HP`
  (params (`Character Target` :type "/Game/Blueprints/Characters/ABaseCharacter Object Reference") (`New Current HP` :type Integer) (`Max HP` :type Integer))
  (bind _asanpccharacter (cast `/Game/Blueprints/Characters/ANPCCharacter` `Character Target`))
  (`/Game/Blueprints/Core/PlayerControllerMaster.Update NPC HP (Own Client)` (`self.Player Controller`) _asanpccharacter `New Current HP` `Max HP`))

(event `self.Stop Collecting (Multicast)`
  (bind _returnvalue (`self.GetComponentByClass` "/Game/Blueprints/Characters/Components/Collecting.Collecting_C"))
  (bind _collectionprogresswidget (`self.CollectionProgressWidget`))
  (`/Engine/EditorBlueprintResources/ActorMacros.Switch Has Authority`
    (:`Authority`
      (`/Engine/EditorBlueprintResources/StandardMacros.IsValid` _returnvalue
        (:`Is Valid`
          (`ActorComponent.K2_DestroyComponent` _returnvalue))))
    (:`Remote`
      (bind _ascollection_progress_widget (cast `/Game/Blueprints/HUD/Collection/CollectionProgressWidget` (`WidgetComponent.GetUserWidgetObject` _collectionprogresswidget)))
      (`Widget.RemoveFromParent` _ascollection_progress_widget)
      (`WidgetComponent.SetWidget` _collectionprogresswidget null))))

(event `/Game/Blueprints/Characters/ICharacter.On Skill Cooldown End (From Server)`
  (params (Skill :type "/Game/Blueprints/Skills/Skill Class Reference"))
  (`/Game/Blueprints/Core/PlayerControllerMaster.On Skill Cooldown End (Server)` (`self.Player Controller`) Skill))

(event `/Game/Blueprints/Characters/ICharacter.On Cast Skill (From Server)`
  (params (Skill :type "/Game/Blueprints/Skills/Skill Class Reference") (Source :type "/Game/Blueprints/Characters/SkillSources Enum" :default "NewEnumerator0"))
  (`/Game/Blueprints/Core/PlayerControllerMaster.On Cast Skill (Own Client)` (`self.Player Controller`) Skill Source))

(event `On Pick Item (Server)`
  (params (`Picked Item` :type "/Game/Blueprints/Interactives/Items/Item_Pickup Object Reference"))
  (bind (_success_ _item_information) (`/Game/Blueprints/Helpers/Helpers.Get Item Information From Datatable` (`/Game/Blueprints/Interactives/Items/Item_Pickup.Item In Datatable` `Picked Item`)))
  (if _success_
    (`/Game/Blueprints/Core/PlayerStateMaster.Add Item To Bag` (`/Game/Blueprints/Core/PlayerControllerMaster.State` (`self.Player Controller`)) _item_information (`/Game/Blueprints/Interactives/Items/Item_Pickup.Amount` `Picked Item`))))

(event `/Game/Blueprints/Characters/ICharacter.On Kill Character`
  (params (`Killed Character` :type "/Game/Blueprints/Characters/ABaseCharacter Class Reference"))
  (bind _asanpccharacter (castclass `/Game/Blueprints/Characters/ANPCCharacter` `Killed Character`))
  (`/Game/Blueprints/Core/PlayerControllerMaster.On Collect Materials (Server)` (`self.Player Controller`) (`.LootMaterials_18_F5A520234DFD06D1D692A8BC2D24D31D` (break `/Game/Blueprints/Characters/NPCs/NPCMetadata` (`/Game/Blueprints/Helpers/Helpers.Get NPC From Datatable` (`.NPC Reference In Datatable` (defaults `/Game/Blueprints/Characters/AHeroCharacter` _asanpccharacter)))))))

(event `/Game/Blueprints/Characters/ICharacter.On Target Dies`
  (`/Game/Blueprints/Core/PlayerControllerMaster.On Target Dies (Own Client)` (`self.Player Controller`)))

(event `/Game/Blueprints/Characters/ICharacter.On Enter Combat (From Server)`
  (`/Game/Blueprints/Core/PlayerControllerMaster.On Enter Combat (Own Client)` (`self.Player Controller`)))

(event `/Game/Blueprints/Characters/ICharacter.On Leave Combat (From Server)`
  (`/Game/Blueprints/Core/PlayerControllerMaster.On Leave Combat (Own Client)` (`self.Player Controller`)))

(fn `Get Target Character`
  (returns (`Success?` :type Boolean) (Character :type "/Game/Blueprints/Characters/ABaseCharacter Object Reference"))
  (bind _asabase_character (cast `/Game/Blueprints/Characters/ABaseCharacter` (`self.Current Target`))
    (:`then`
      (return true _asabase_character))
    (:`CastFailed`
      (return false null))))

(fn `GetPlayerCamera`
  (returns (Camera :type "CameraComponent Object Reference"))
  (return null))

(fn `Give Items To Other Character`
  (params (`Killer Character` :type "/Game/Blueprints/Characters/ABaseCharacter Object Reference"))
  (bind _player_controller (`self.Player Controller`))
  (bind _state (`/Game/Blueprints/Core/PlayerControllerMaster.State` _player_controller))
  (bind _items (`/Game/Blueprints/Core/PlayerStateMaster.Get All Items` (`/Game/Blueprints/Core/PlayerControllerMaster.State` (`self.Player Controller`))))
  (if (> (`KismetArrayLibrary.Array_Length` _items) 0)
    (`|SpawnActorFromClass` "/Game/Blueprints/Interactives/Chests/ACharacterChest.ACharacterChest_C" (`SceneComponent.K2_GetComponentToWorld` (`self.Mesh`)) "AlwaysSpawn" "OverrideRootScale" null _items null))
  (if (`/Game/Blueprints/Core/PlayerStateMaster.Has Any Material?` _state)
    (bind _asahero_character (cast `/Game/Blueprints/Characters/AHeroCharacter` (`local.Killer Character`))
      (:`then`
        (`/Game/Blueprints/Core/PlayerControllerMaster.Transport Materials To Other Player (Server)` _player_controller (`/Game/Blueprints/Core/PlayerStateMaster.Materials` _state) _asahero_character))
      (:`CastFailed`
        _)))
  (`/Game/Blueprints/Core/PlayerStateMaster.Remove All Resources From Bags` (`/Game/Blueprints/Core/PlayerControllerMaster.State` (`self.Player Controller`))))

(fn `Grant XP`
  (params (Amount :type Integer))
  (`self.Increase Current XP` Amount))

(fn `Is In Interaction Range?`
  (params (Interactive :type "/Game/Blueprints/Interactives/AInteractive Object Reference"))
  (returns (`Is In Interaction Range?` :type Boolean))
  (return (<= (- (`self.GetDistanceTo` (`local.Interactive`)) (+ (`SphereComponent.SphereRadius` (`/Game/Blueprints/Interactives/AInteractive.Borders` Interactive)) (`CapsuleComponent.CapsuleRadius` (`self.CapsuleComponent`)))) 200.0)))

(fn `Start Cast Progress Widget`
  (params (Duration :type "Float (double-precision)"))
  (bind _returnvalue (`|CreateWidget` "/Game/Blueprints/HUD/Collection/CollectionProgressWidget.CollectionProgressWidget_C" null Duration))
  (`WidgetComponent.SetWidget` (`self.CollectionProgressWidget`) _returnvalue))

(fn `UserConstructionScript`
  (`parent.UserConstructionScript`))