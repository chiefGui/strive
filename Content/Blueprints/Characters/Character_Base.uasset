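; Base character for a networked RPG, handling AI movement, targeted combat, HP and mana, stats, death and XP.
; Server-side repeaters drive target or idle logic and per-second regen until death.
; Animation events resolve hits on the server as Strength minus PhysicalDefense, then multicast results for remote damage widgets and server death handling.
; Server hook events expose state changes, stat functions adjust attributes, and an XP DataTable determines levels.
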(event `On Enter Fog (Own Client)`
  (`SceneComponent.SetVisibility` (`self.CapsuleComponent`) true true))

(event `self.ReceiveBeginPlay`
  (`/Engine/EditorBlueprintResources/ActorMacros.Switch Has Authority`
    (:`Authority`
      (`|ExecutionSequence`
        (:`then_0`
          (`/Game/Blueprints/Helpers/Time_Macros.Repeater` 0.1 :!label _label
            (:`On Every Interval`
              (if (`self.Is Dead?`)
                (goto _label :!via `Stop`)
                (else
                  (`/Engine/EditorBlueprintResources/StandardMacros.IsValid` (`self.Current Target`)
                    (:`Is Valid`
                      (`/Game/Blueprints/Characters/I_Character.While Target Is Valid (Server)`))
                    (:`Is Not Valid`
                      (set `self.Is Attacking?` false)
                      (if (and (not (`self.Is Attacking?`)) (not (`self.Is Walking?`)) (not (`self.Is Dead?`)) (not (`self.Is Casting?`)))
                        (`/Game/Blueprints/Characters/I_Character.On Idle (Server)`)))))))))
        (:`then_1`
          (`/Game/Blueprints/Helpers/Time_Macros.Repeater` 1.0 :!label _label_2
            (:`On Every Interval`
              (if (`self.Is Dead?`)
                (goto _label_2 :!via `Stop`)
                (else
                  (`|ExecutionSequence`
                    (:`then_0`
                      (if (`self.Should Regen HP?`)
                        (`self.Increase HP` (`self.HP Regen Per Second`))))
                    (:`then_1`
                      (if (`self.Should Regen Mana?`)
                        (`self.Increase Mana` (`self.Mana Regen Per Second`))))))))))))))

(event `On Hit Success`
  ;[1 1 1] Animation Events
  (`/Engine/EditorBlueprintResources/ActorMacros.Switch Has Authority`
    (:`Authority`
      (`self.Resolve Attack On Current Target (On Server)`))))

(event `Move To Destination (Server)`
  (params (`Destination Location` :type "Vector Structure") (`Destination Actor` :type "Actor Object Reference"))
  (`|AIMoveTo` self `Destination Location` (`self.Current Target`)
    (:`then`
      (set `self.Is Walking?` true)
      (set `self.Is Attacking?` false))
    (:`OnSuccess`
      (set `self.Is Walking?` false)
      (`/Game/Blueprints/Characters/I_Character.On Reached Destination (Server)`))
    (:`OnFail`
      (set `self.Is Walking?` false))))

(event `On Hit Ended`
  ;[1 1 1] Animation Events
  (`/Engine/EditorBlueprintResources/ActorMacros.Switch Has Authority`
    (:`Authority`
      (`self.Look At Current Target`)
      (if (not (`self.Is Current Target Within Attack Range?`))
        (set `self.Is Attacking?` false)
        (`self.Move Towards Current Target`)))))

(event `On Death Animation Has Ended`
  ;[1 1 1] Animation Events
  (`/Engine/EditorBlueprintResources/ActorMacros.Switch Has Authority`
    (:`Authority`
      (`self.After Death Animation (Server)`))))

(event `Die (Server)`
  (params (`Killer Character` :type "/Game/Blueprints/Characters/Character_Base Object Reference"))
  ;[1 1 1] On Death
  (`self.Stop Movements`)
  (set `self.Is Walking?` false)
  (set `self.Is Attacking?` false)
  (set `self.Is Dead?` true)
  (set `self.Current Target` null)
  (`self.On Death (Server)` `Killer Character`))

(event `On Kill A Target (Server)`
  (params (`Target Killed` :type "/Game/Blueprints/Characters/Character_Base Class Reference"))
  ;[1 1 1] When Character killed its target
  (`/Engine/EditorBlueprintResources/ActorMacros.Switch Has Authority`
    (:`Authority`
      (set `self.Is Attacking?` false)
      (set `self.Is Walking?` false)
      (set `self.Current Target` null)
      (`/Game/Blueprints/Characters/I_Character.After Kill Character (Server)` `Target Killed`))))

(event `Respond To Interaction`
  (params (`Trigger Character` :type "/Game/Blueprints/Characters/Character_Base Object Reference"))
  ;[1 1 1] Respond to interaction
  (`self.On Respond To Interaction` `Trigger Character`))

(event `Attack Actor`
  (params (Actor :type "Actor Object Reference"))
  ;[1 1 1] Start attacking
  (if (not (`self.Is Attacking?`))
    (set `self.Is Attacking?` true)
    (`self.Stop Movements`)
    (`self.Look At Actor` Actor)))

(event `On Attacked (Multicast)`
  (params (Attacker :type "/Game/Blueprints/Characters/Character_Base Object Reference") (`Has Died?` :type Boolean) (`Damage Taken` :type Integer) (`New Current HP` :type Integer))
  ;[1 1 1] On HP decreased
  (`/Engine/EditorBlueprintResources/ActorMacros.Switch Has Authority`
    (:`Authority`
      (if `Has Died?`
        (`self.Die (Server)` Attacker)
        (else
          (`self.On Attacked (Server)` Attacker))))
    (:`Remote`
      (`self.Show Damage Widget` `Damage Taken`))))

(fn `Attack Current Target`
  (bind _ascharacter_base (cast `/Game/Blueprints/Characters/Character_Base` (`self.Current Target`)))
  (if (`/Game/Blueprints/Characters/Character_Base.Is Dead?` _ascharacter_base)
    (set `self.Is Attacking?` false)
    (set `self.Current Target` null)
    (else
      (`self.Attack Actor` (`self.Current Target`)))))

(fn `Calculate Physical Damage Against Character`
  (params (Character :type "/Game/Blueprints/Characters/Character_Base Object Reference"))
  (returns (Damage :type Integer))
  (return (`KismetMathLibrary.Clamp` (- (`KismetMathLibrary.Round` (`self.Strength`)) (`/Game/Blueprints/Characters/Character_Base.Physical Defense` Character)) 1 99999)))

(fn `Decrease Attack Speed`
  (params (Amount :type "Float (double-precision)"))
  (returns (`New Attack Speed` :type "Float (double-precision)"))
  (bind _output_get (set `self.Attack Speed` (- (`self.Attack Speed`) Amount)))
  (return _output_get))

(fn `Decrease Attack Speed By Percentage`
  (params (Percentage :type "Float (double-precision)"))
  (returns (`New Attack Speed` :type "Float (double-precision)"))
  (bind _output_get (set `self.Attack Speed` (- (`self.Attack Speed`) (/ (* (`self.Attack Speed`) Percentage) 100.0))))
  (return _output_get))

(fn `Decrease HP`
  (params (Amount :type Integer))
  (returns (`New Current HP` :type Integer) (`Has Died?` :type Boolean))
  (bind _max_hp (`self.Max HP`))
  (bind _output_get (set `self.Current HP` (`KismetMathLibrary.Clamp` (- (`self.Current HP`) Amount) 0 _max_hp)))
  (`/Game/Blueprints/Characters/I_Character.On HP Is Updated (Server)` (`local.Amount`) _output_get _max_hp)
  (return _output_get (<= (`self.Current HP`) 0)))

(fn `Decrease HP Regen Per Second`
  (params (Amount :type Integer))
  (returns (`New HP Regen Per Second` :type Integer))
  (bind _output_get (set `self.HP Regen Per Second` (`KismetMathLibrary.Clamp` (- (`self.HP Regen Per Second`) Amount) 0 99999)))
  (return _output_get))

(fn `Decrease Mana`
  (params (Amount :type Integer))
  (returns (`New Current Mana` :type Integer))
  (bind _max_mana (`self.Max Mana`))
  (bind _output_get (set `self.Current Mana` (`KismetMathLibrary.Clamp` (- (`self.Current Mana`) Amount) 0 _max_mana)))
  (`/Game/Blueprints/Characters/I_Character.On Mana Is Updated (Server)` (`local.Amount`) _output_get _max_mana)
  (return _output_get))

(fn `Decrease Mana Regen Per Second`
  (params (Amount :type Integer))
  (returns (`New Mana Regen Per Second` :type Integer))
  (bind _output_get (set `self.Mana Regen Per Second` (`KismetMathLibrary.Clamp` (- (`self.Mana Regen Per Second`) Amount) 0 99999)))
  (return _output_get))

(fn `Decrease Max HP`
  (params (Amount :type Integer))
  (returns (`New Max HP` :type Integer))
  (bind _output_get (set `self.Max HP` (- (`self.Max HP`) Amount)))
  (if (>= (`self.Current HP`) _output_get)
    (set `self.Current HP` _output_get))
  (`/Game/Blueprints/Characters/I_Character.On HP Is Updated (Server)` 0 (`self.Current HP`) (`self.Max HP`))
  (return (`self.Max HP`)))

(fn `Decrease Max Mana`
  (params (Amount :type Integer))
  (returns (`New Max Mana` :type Integer))
  (bind _output_get (set `self.Max Mana` (- (`self.Max Mana`) Amount)))
  (if (>= (`self.Current Mana`) _output_get)
    (set `self.Current Mana` _output_get))
  (`/Game/Blueprints/Characters/I_Character.On Mana Is Updated (Server)` 0 (`self.Current Mana`) _output_get)
  (return _output_get))

(fn `Decrease Physical Defense`
  (params (Amount :type Integer))
  (returns (Output_Get :type Integer))
  (bind _output_get (set `self.Physical Defense` (`KismetMathLibrary.Clamp` (- (`self.Physical Defense`) Amount) 0 9999)))
  (return _output_get))

(fn `Decrease Strength`
  (params (Amount :type "Float (double-precision)"))
  (returns (`New Strength` :type "Float (double-precision)"))
  (bind _output_get (set `self.Strength` (- (`self.Strength`) Amount)))
  (return _output_get))

(fn `Decrease Walk Speed`
  (params (Amount :type "Float (double-precision)"))
  (returns (`New Walk Speed` :type "Float (double-precision)"))
  (bind _output_get (set `CharacterMovementComponent.MaxWalkSpeed` (- (`CharacterMovementComponent.MaxWalkSpeed` (`self.CharacterMovement`)) Amount) (`self.CharacterMovement`)))
  (return _output_get))

(fn `Every Frame Logic`)

(fn `Get Current Level`
  (returns (`Current Level` :type Integer))
  (locals (`Local Current Level` :type Integer))
  (bind _outrownames (`DataTableFunctionLibrary.GetDataTableRowNames` "/Game/Blueprints/Characters/Heroes/Leveling/XPTable.XPTable"))
  (for _array_element _outrownames
    (bind _returnvalue (`|GetDataTableRow` "/Game/Blueprints/Characters/Heroes/Leveling/XPTable.XPTable" _array_element)
      (:`then`
        (bind (_level _xpneeded) (break `/Game/Blueprints/Characters/Heroes/Leveling/LevelStructure` _returnvalue))
        (if (<= (`self.Current XP`) _xpneeded)
          (set `local.Local Current Level` _level)
          (break)))))
  (return (`local.Local Current Level`)))

(fn `Get Distance To Other Character`
  (params (`Other Character` :type "/Game/Blueprints/Characters/Character_Base Object Reference"))
  (returns (Distance :type "Float (double-precision)"))
  (return (- (`self.GetDistanceTo` (`local.Other Character`)) (+ (`CapsuleComponent.CapsuleRadius` (`Character.CapsuleComponent` `Other Character`)) (`CapsuleComponent.CapsuleRadius` (`self.CapsuleComponent`))))))

(fn `Increase Attack Speed`
  (params (Amount :type "Float (double-precision)"))
  (returns (`New Attack Speed` :type "Float (double-precision)"))
  (bind _output_get (set `self.Attack Speed` (+ Amount (`self.Attack Speed`))))
  (return _output_get))

(fn `Increase Attack Speed By Percentage`
  (params (Percentage :type "Float (double-precision)"))
  (returns (`New Attack Speed` :type "Float (double-precision)"))
  (bind _output_get (set `self.Attack Speed` (+ (`self.Attack Speed`) (/ (* (`self.Attack Speed`) Percentage) 100.0))))
  (return _output_get))

(fn `Increase HP`
  (params (Amount :type Integer))
  (returns (`New Current HP` :type Integer))
  (bind _max_hp (`self.Max HP`))
  (bind _output_get (set `self.Current HP` (`KismetMathLibrary.Clamp` (+ Amount (`self.Current HP`)) 0 _max_hp)))
  (`/Game/Blueprints/Characters/I_Character.On HP Is Updated (Server)` (`local.Amount`) _output_get _max_hp true)
  (return _output_get))

(fn `Increase HP Regen Per Second`
  (params (Amount :type Integer))
  (returns (`New HP Regen Per Second` :type Integer))
  (bind _output_get (set `self.HP Regen Per Second` (+ Amount (`self.HP Regen Per Second`))))
  (return _output_get))

(fn `Increase Mana`
  (params (Amount :type Integer))
  (returns (`New Current Mana` :type Integer))
  (bind _max_mana (`self.Max Mana`))
  (bind _output_get (set `self.Current Mana` (`KismetMathLibrary.Clamp` (+ Amount (`self.Current Mana`)) 0 _max_mana)))
  (`self.On Mana Is Updated (Server)` (`local.Amount`) _output_get _max_mana true)
  (return _output_get))

(fn `Increase Mana Regen Per Second`
  (params (Amount :type Integer))
  (returns (`New Mana Regen Per Second` :type Integer))
  (bind _output_get (set `self.Mana Regen Per Second` (+ Amount (`self.Mana Regen Per Second`))))
  (return _output_get))

(fn `Increase Max HP`
  (params (Amount :type Integer))
  (returns (`New Max HP` :type Integer))
  (bind _output_get (set `self.Max HP` (+ Amount (`self.Max HP`))))
  (`self.On HP Is Updated (Server)` 0 (`self.Current HP`) _output_get true)
  (return _output_get))

(fn `Increase Max Mana`
  (params (Amount :type Integer))
  (returns (`New Max Mana` :type Integer))
  (bind _output_get (set `self.Max Mana` (+ Amount (`self.Max Mana`))))
  (`self.On Mana Is Updated (Server)` 0 (`self.Current Mana`) _output_get true)
  (return _output_get))

(fn `Increase Physical Defense`
  (params (Amount :type Integer))
  (returns (`New Physical Defense` :type Integer))
  (bind _output_get (set `self.Physical Defense` (+ (`self.Physical Defense`) Amount)))
  (return _output_get))

(fn `Increase Strength`
  (params (Amount :type "Float (double-precision)"))
  (returns (`New Strength` :type "Float (double-precision)"))
  (bind _output_get (set `self.Strength` (+ Amount (`self.Strength`))))
  (return _output_get))

(fn `Increase Walk Speed`
  (params (Amount :type "Float (double-precision)"))
  (returns (`New Walk Speed` :type "Float (double-precision)"))
  (bind _output_get (set `CharacterMovementComponent.MaxWalkSpeed` (+ Amount (`CharacterMovementComponent.MaxWalkSpeed` (`self.CharacterMovement`))) (`self.CharacterMovement`)))
  (return _output_get))

(fn `Increase XP`
  (params (Amount :type Integer))
  (returns (`New XP` :type Integer) (`Levels Obtained` :type Integer))
  (locals (`Local Levels Obtained` :type Integer) (`Local New XP` :type Integer))
  (set `local.Local New XP` (+ Amount (`self.Current XP`)))
  (bind _outrownames (`DataTableFunctionLibrary.GetDataTableRowNames` "/Game/Blueprints/Characters/Heroes/Leveling/XPTable.XPTable"))
  (for _array_element _outrownames
    (bind _returnvalue (`|GetDataTableRow` "/Game/Blueprints/Characters/Heroes/Leveling/XPTable.XPTable" _array_element)
      (:`then`
        (bind (_level _xpneeded) (break `/Game/Blueprints/Characters/Heroes/Leveling/LevelStructure` _returnvalue))
        (if (> _xpneeded (`self.Current XP`))
          (if (>= (`local.Local New XP`) _xpneeded)
            (`/Engine/EditorBlueprintResources/StandardMacros.IncrementInt` (`local.Local Levels Obtained`)))))))
  (set `self.Current XP` (`local.Local New XP`))
  (return (`local.Local New XP`) (`local.Local Levels Obtained`)))

(fn `Is Aggressive Against Actor?`
  (params (Actor :type "Actor Object Reference"))
  (returns (`Is Aggressive?` :type Boolean))
  (locals (`_Is Aggressive?` :type Boolean))
  (for _array_element (`self.Aggressive Against`)
    (bind _outactors (`GameplayStatics.GetAllActorsOfClass` _array_element))
    (bind _ascharacter_base (cast `/Game/Blueprints/Characters/Character_Base` (`local.Actor`)))
    (if (!= (`KismetArrayLibrary.Array_Find` _outactors _ascharacter_base) -1)
      (set `local._Is Aggressive?` true)
      (break)))
  (return (`local._Is Aggressive?`)))

(fn `Is Aggressive Against Current Target?`
  (returns (`Is Aggressive?` :type Boolean))
  (locals (`IsAggressive?` :type Boolean))
  (return (`self.Is Aggressive Against Actor?` (`self.Current Target`))))

(fn `Is Current Target Dead?`
  (returns (`IsDead?` :type Boolean))
  (bind _ascharacter_base (cast `/Game/Blueprints/Characters/Character_Base` (`self.Current Target`)))
  (return (`/Game/Blueprints/Characters/Character_Base.Is Dead?` _ascharacter_base)))

(fn `Is Current Target Within Attack Range?`
  (returns (`In Range?` :type Boolean))
  (bind _ascharacter_base (cast `/Game/Blueprints/Characters/Character_Base` (`self.Current Target`)))
  (return (<= (`self.Get Distance To Other Character` _ascharacter_base) (`self.Attack Range`))))

(fn `Is Current Target, Myself?`
  (returns (ReturnValue :type Boolean))
  (return (== (`self.Current Target`) self)))

(fn `Is Moving?`
  (returns (`IsMoving?` :type Boolean))
  (return (> (`KismetMathLibrary.VSize` (`self.GetVelocity`)) 0.0)))

(fn `Look At Actor`
  (params (Actor :type "Actor Object Reference"))
  (`/Engine/EditorBlueprintResources/StandardMacros.IsValid` Actor
    (:`Is Valid`
      (`self.Look At Location` (`SceneComponent.K2_GetComponentLocation` (`Actor.RootComponent` Actor))))))

(fn `Look At Current Target`
  (bind _current_target (`self.Current Target`))
  (`/Engine/EditorBlueprintResources/StandardMacros.IsValid` _current_target
    (:`Is Valid`
      (`self.Look At Location` (`SceneComponent.K2_GetComponentLocation` (`Actor.RootComponent` _current_target))))))

(fn `Look At Location`
  (params (Location :type "Vector Structure"))
  (bind (_returnvalue_roll _returnvalue_pitch _returnvalue_yaw) (`KismetMathLibrary.BreakRotator` (`KismetMathLibrary.FindLookAtRotation` (`SceneComponent.K2_GetComponentLocation` (`self.Mesh`)) Location)))
  (`self.K2_SetActorRotation` (`KismetMathLibrary.MakeRotator` 0.0 0.0 _returnvalue_yaw)))

(fn `Move Towards Current Target`
  (bind _current_target (`self.Current Target`))
  (if (not (`self.Is Attacking?`))
    (`/Engine/EditorBlueprintResources/StandardMacros.IsValid` _current_target
      (:`Is Valid`
        (`self.Move To Destination (Server)` (`SceneComponent.K2_GetComponentLocation` (`Actor.RootComponent` _current_target)))))))

(fn `Resolve Attack On Current Target (On Server)`
  (locals (`Target Character` :type "/Game/Blueprints/Characters/Character_Base Object Reference"))
  (bind _target_character (`local.Target Character`))
  (bind _damage (`self.Calculate Physical Damage Against Character` _target_character))
  (bind _ascharacter_base (cast `/Game/Blueprints/Characters/Character_Base` (`self.Current Target`)))
  (bind _output_get (set `local.Target Character` _ascharacter_base))
  (if (`/Game/Blueprints/Characters/Character_Base.Is Dead?` _output_get)
    (set `self.Current Target` null)
    (set `self.Is Attacking?` false)
    (set `self.Is Walking?` false)
    (set `self.Is Sat?` false)
    (`self.Stop Movements`)
    (else
      (bind (_new_current_hp _has_died_) (`self.Decrease HP` _target_character _damage))
      (`self.On Attacked (Multicast)` (`local.Target Character`) self _has_died_ _damage _new_current_hp)
      (if _has_died_
        (`self.On Kill A Target (Server)` (`GameplayStatics.GetObjectClass` (`local.Target Character`)))))))

(fn `Should Regen HP?`
  (returns (ReturnValue :type Boolean))
  (return (< (`self.Current HP`) (`self.Max HP`))))

(fn `Should Regen Mana?`
  (returns (ReturnValue :type Boolean))
  (return (< (`self.Current Mana`) (`self.Max Mana`))))

(fn `Show Damage Widget`
  (params (Amount :type Integer))
  (bind _returnvalue (`|CreateWidget` "/Game/Blueprints/Characters/Character_Damage_Widget.Character_Damage_Widget_C" null Amount self))
  (`UserWidget.AddToViewport` _returnvalue 0))

(fn `Stop Movements`
  (`MovementComponent.StopMovementImmediately` (`self.CharacterMovement`))
  (set `self.Is Walking?` false))

(fn `UserConstructionScript`)