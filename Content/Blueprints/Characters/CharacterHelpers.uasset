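; Helper functions for querying characters: range, alliance, death XP, master lookup and attribute values.
; Max range scales the physical attack range by a tiered multiplier that shrinks as range grows.
; Alliance and master checks rely on actor ownership, treating owner and owned, or characters sharing an owner, as allies.
; Death XP comes from the character's datatable row, and a modifier switch returns the matching attribute's current value as a number.
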(fn `Are Characters Allied?`
  (params (`Character 1` :type "/Game/Blueprints/Characters/ABaseCharacter Object Reference") (`Character 2` :type "/Game/Blueprints/Characters/ABaseCharacter Object Reference"))
  (returns (`Return Value` :type Boolean))
  (if (== (`Actor.GetOwner` (`local.Character 1`)) (`local.Character 2`))
    (return true)
    (elif (== (`local.Character 1`) (`Actor.GetOwner` (`local.Character 2`)))
      (return true)
      (elif (== (`Actor.GetOwner` (`local.Character 1`)) (`Actor.GetOwner` (`local.Character 2`)))
        (return true)
        (else
          (return false))))))

(fn `Character Has Master?`
  (params (Character :type "/Game/Blueprints/Characters/ABaseCharacter Object Reference"))
  (returns (`Success?` :type Boolean) (`Master Character` :type "/Game/Blueprints/Characters/ABaseCharacter Object Reference"))
  (bind _asabase_character (cast `/Game/Blueprints/Characters/ABaseCharacter` (`Actor.GetOwner` Character))
    (:`then`
      (return true _asabase_character))
    (:`CastFailed`
      (return false null))))

(fn `Get Attribute State By Modifier`
  (params (Character :type "/Game/Blueprints/Characters/ABaseCharacter Object Reference") (Modifier :type "/Game/Blueprints/Characters/Modifiers Enum" :default "NewEnumerator17"))
  (returns (`Attribute Current Amount` :type "Float (double-precision)"))
  (locals (`Final Amount` :type "Float (double-precision)"))
  (switch `/Game/Blueprints/Characters/Modifiers` Modifier
    (:`NewEnumerator0`
      (set `local.Final Amount` (`KismetMathLibrary.Conv_IntToDouble` (`.Current` (`/Game/Blueprints/Characters/ABaseCharacter.Get Max HP` (`local.Character`))))))
    (:`NewEnumerator1`
      (set `local.Final Amount` (`KismetMathLibrary.Conv_IntToDouble` (`.Current` (`/Game/Blueprints/Characters/ABaseCharacter.Get Max MP` (`local.Character`))))))
    (:`NewEnumerator2`
      (set `local.Final Amount` (`.Current` (`/Game/Blueprints/Characters/ABaseCharacter.Get HP Regen` (`local.Character`)))))
    (:`NewEnumerator3`
      (set `local.Final Amount` (`.Current` (`/Game/Blueprints/Characters/ABaseCharacter.Get MP Regen` (`local.Character`)))))
    (:`NewEnumerator4`
      (set `local.Final Amount` (`.Current` (`/Game/Blueprints/Characters/ABaseCharacter.Get Physical Damage` (`local.Character`)))))
    (:`NewEnumerator5`
      (set `local.Final Amount` (`.Current` (`/Game/Blueprints/Characters/ABaseCharacter.Get Physical Defense` (`local.Character`)))))
    (:`NewEnumerator15`
      (set `local.Final Amount` (`.Current` (`/Game/Blueprints/Characters/ABaseCharacter.Get Magical Damage` (`local.Character`)))))
    (:`NewEnumerator16`
      (set `local.Final Amount` (`.Current` (`/Game/Blueprints/Characters/ABaseCharacter.Get Magical Defense` (`local.Character`)))))
    (:`NewEnumerator8`
      (set `local.Final Amount` (`.Current` (`/Game/Blueprints/Characters/ABaseCharacter.Get Neutral Physical Damage` (`local.Character`)))))
    (:`NewEnumerator6`
      (set `local.Final Amount` (`.Current` (`/Game/Blueprints/Characters/ABaseCharacter.Get ASPD` (`local.Character`)))))
    (:`NewEnumerator7`
      (set `local.Final Amount` (`.Current` (`/Game/Blueprints/Characters/ABaseCharacter.Get Walk Speed` (`local.Character`)))))
    (:`NewEnumerator10`
      (set `local.Final Amount` (`.Current` (`/Game/Blueprints/Characters/ABaseCharacter.Get Strength` (`local.Character`)))))
    (:`NewEnumerator11`
      (set `local.Final Amount` (`.Current` (`/Game/Blueprints/Characters/ABaseCharacter.Get Agility` (`local.Character`)))))
    (:`NewEnumerator12`
      (set `local.Final Amount` (`.Current` (`/Game/Blueprints/Characters/ABaseCharacter.Get Intelligence` (`local.Character`)))))
    (:`NewEnumerator13`
      (set `local.Final Amount` (`.Current` (`/Game/Blueprints/Characters/ABaseCharacter.Get Vitality` (`local.Character`))))))
  (return (`local.Final Amount`)))

(fn `Get Character Death XP`
  (params (Character :type "/Game/Blueprints/Characters/ABaseCharacter Object Reference"))
  (returns (`Death XP` :type Integer))
  (return (`.BaseDeathXP_62_B189C1414C3DBD492EAFF18E6A00AFAF` (break `/Game/Blueprints/Characters/CharacterMetadata` (`/Game/Blueprints/Helpers/Helpers.Get Character From Datatable` (`/Game/Blueprints/Characters/ABaseCharacter.Character Reference In Datatable` Character))))))

(fn `Get Max Range`
  (params (Character :type "/Game/Blueprints/Characters/ABaseCharacter Object Reference"))
  (returns (`Max Range` :type "Float (double-precision)"))
  (locals (Multiplier :type "Float (double-precision)"))
  (bind _current_physical_attack_range (`/Game/Blueprints/Characters/ABaseCharacter.Get Current Physical Attack Range` Character))
  (if (<= _current_physical_attack_range 100.0)
    (set `local.Multiplier` 5.0)
    (elif (<= _current_physical_attack_range 200.0)
      (set `local.Multiplier` 4.0)
      (elif (<= _current_physical_attack_range 300.0)
        (set `local.Multiplier` 3.0)
        (elif (<= _current_physical_attack_range 1000.0)
          (set `local.Multiplier` 3.0)
          (else
            (set `local.Multiplier` 2.0))))))
  (return (* (`/Game/Blueprints/Characters/ABaseCharacter.Get Current Physical Attack Range` (`local.Character`)) (`local.Multiplier`))))