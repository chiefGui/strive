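; AProjectile is a homing projectile fired by a Character_Base at a specific target character.
; On BeginPlay the server stores its owner as the origin and passes the target to PropagateProjectile, which sets it as the movement component's homing target.
; On the server, overlapping that target reports the hit back to the origin character and destroys the projectile; other overlaps are ignored.
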(event `self.ReceiveBeginPlay`
  (`/Engine/EditorBlueprintResources/ActorMacros.Switch Has Authority`
    (:`Authority`
      (bind _ascharacter_base (cast `/Game/Blueprints/Characters/Character_Base` (`self.GetOwner`)))
      (set `self.Origin Character` _ascharacter_base)
      (`self.Propagate Projectile` (`self.Target Character`)))))

(event `Propagate Projectile`
  (params (Target :type "/Game/Blueprints/Characters/Character_Base Object Reference"))
  (set `ProjectileMovementComponent.HomingTargetComponent` (`Actor.RootComponent` Target) (`self.ProjectileMovement`)))

(event `self.Collision Sphere.OnComponentBeginOverlap`
  (params (OverlappedComponent :type "PrimitiveComponent Object Reference") (OtherActor :type "Actor Object Reference") (OtherComp :type "PrimitiveComponent Object Reference") (OtherBodyIndex :type Integer) (bFromSweep :type Boolean) (SweepResult :type "HitResult Structure (by ref)"))
  (`/Engine/EditorBlueprintResources/ActorMacros.Switch Has Authority`
    (:`Authority`
      (if (== OtherActor (`self.Target Character`))
        (`/Game/Blueprints/Characters/Character_Base.On Projectile Hit Target Character` (`self.Origin Character`) (`self.Target Character`))
        (`self.K2_DestroyActor`)))))

(fn `UserConstructionScript`)