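; AChest is a lootable chest Blueprint that spawns random item drops when opened.
; The Server.Open event checks IsOpened, rolls the Loot data through GetRandomDrop, and spawns each returned class at the same point in front of the chest.
; IsOpened is set inside the spawn loop, so a roll that yields no items leaves the chest openable again.
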(event `Open (Server)`
  (if (not (`self.Is Opened?`))
    (bind (_looted_items _has_looted_something_) (`/Game/Blueprints/Helpers/LootFunctions.Get Random Drop` (`self.Loot`)))
    (if _has_looted_something_
      (for _array_element _looted_items
        (`|SpawnActorFromClass` _array_element (`KismetMathLibrary.Conv_VectorToTransform` (+ (`self.K2_GetActorLocation`) (* (`self.GetActorForwardVector`) 150.0))) "Undefined" "OverrideRootScale" null 1 null)
        (set `self.Is Opened?` true)))))

(fn `UserConstructionScript`)