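; Short-lived component that runs the cooldown for a single skill on its owning PlayerControllerMaster.
; After a tiny BeginPlay delay, if the skill is enabled, it reports the skill state to the owning client and starts a one-shot timer using the skill's data table cooldown time.
; On expiry it clears the cooldown through the controller, reports the new state and destroys itself.
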(event `self.ReceiveBeginPlay`
  (bind _skill_with_state (`self.Skill With State`))
  (bind (_skill _isincooldown_ _isenabled_) (break `/Game/Blueprints/Skills/SkillWithState` _skill_with_state))
  (bind _asplayer_controller_master (cast `/Game/Blueprints/Core/PlayerControllerMaster` (`self.GetOwner`)))
  (set `self.Player Controller` _asplayer_controller_master)
  (`KismetSystemLibrary.Delay` 0.001)
  (if _isenabled_
    (`/Game/Blueprints/Core/PlayerControllerMaster.On Skill State Has Changed (Owning Client)` (`self.Player Controller`) _skill_with_state)
    (`KismetSystemLibrary.K2_SetTimerDelegate` (delegate `Remove Cooldown`) (`.CooldownTime_23_A1647BEE4F8D340CD88EADB96F6D6D75` (break `/Game/Blueprints/Skills/SkillMetadata` (`/Game/Blueprints/Helpers/Helpers.Get Skill Information From Datatable` (defaults `/Game/Blueprints/Core/PlayerControllerMaster` _skill)))))))

(event `Remove Cooldown`
  (bind _new_skill_with_state (`/Game/Blueprints/Core/PlayerControllerMaster.Set Cooldown For Skill` (`self.Player Controller`) (`.Skill_3_01C3ED4C4A86F0F2FC12D09B6FAEBC11` (break `/Game/Blueprints/Skills/SkillWithState` (`self.Skill With State`))) false))
  (`/Game/Blueprints/Core/PlayerControllerMaster.On Skill State Has Changed (Owning Client)` (`self.Player Controller`) _new_skill_with_state)
  (`self.K2_DestroyComponent`))