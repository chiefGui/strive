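; Base Blueprint for static summons owned by a master character, with empty server and multicast hooks for subclasses.
; Construction caches the owning character as master and derives its damage contribution from the ScalesWith attribute.
; The server fires summon events, optionally expires the actor after LifeDuration, and routes territory-sphere overlaps by living characters into ally or enemy events.
; Helpers handle owner-only mesh visibility and notifying the master on destruction.
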(event `self.ReceiveBeginPlay`
  (`/Engine/EditorBlueprintResources/ActorMacros.Switch Has Authority`
    (:`Authority`
      (`self.On Summoned (Server)`)
      (`self.On Summoned (Multicast)`)
      (if (> (`self.Life Duration`) 0.0)
        (`KismetSystemLibrary.Delay` (`self.Life Duration`))
        (`self.K2_DestroyActor`)))))

(event `On Summoned (Server)`)

(event `On Summoned (Multicast)`)

(event `Make Visible (Multicast)`
  (params (Mesh :type "MeshComponent Object Reference"))
  (`self.Make Only Visible To Owner` Mesh))

(event `self.TerritoryCollisionSphere.OnOtherCharacterBeginOverlap`
  (params (OtherCharacter :type "OnlineCharacter Object Reference"))
  (`/Engine/EditorBlueprintResources/ActorMacros.Switch Has Authority`
    (:`Authority`
      (bind _asabase_character (cast `/Game/Blueprints/Characters/ABaseCharacter` OtherCharacter))
      (if (`/Game/Blueprints/Characters/ABaseCharacter.Is Dead?` _asabase_character)
        _
        (elif (`/Game/Blueprints/Characters/CharacterHelpers.Are Characters Allied?` _asabase_character (`self.Master Character`))
          (`self.On Ally Begin Overlap (Server)` _asabase_character)
          (else
            (`self.On Enemy Begin Overlap (Server)` _asabase_character)
            (`self.On Enemy Begin Overlap (Multicast)` _asabase_character)))))))

(event `On Ally Begin Overlap (Server)`
  (params (`Ally Character` :type "/Game/Blueprints/Characters/ABaseCharacter Object Reference")))

(event `On Enemy Begin Overlap (Server)`
  (params (`Enemy Character` :type "/Game/Blueprints/Characters/ABaseCharacter Object Reference")))

(event `On Enemy Begin Overlap (Multicast)`
  (params (`Enemy Character` :type "/Game/Blueprints/Characters/ABaseCharacter Object Reference")))

(event `Destroy (Server)`
  (`/Game/Blueprints/Characters/ABaseCharacter.Destroy Ally (Server)` (`self.Master Character`) self)
  (`self.On Destroy (Server)`))

(event `On Destroy (Server)`)

(event `On Destroy (Multicast)`)

(fn `Make Only Visible To Owner`
  (params (`Mesh Component` :type "MeshComponent Object Reference"))
  (`PrimitiveComponent.SetOnlyOwnerSee` `Mesh Component` true))

(fn `UserConstructionScript`
  (bind _asabase_character (cast `/Game/Blueprints/Characters/ABaseCharacter` (`self.GetOwner`)))
  (bind _output_get (set `self.Master Character` _asabase_character))
  (set `self.Character Damage Contribution` (`/Game/Blueprints/Characters/CharacterHelpers.Get Attribute State By Modifier` _output_get (`self.Scales With`))))