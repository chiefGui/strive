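; Obstacle-avoidance component that changes its owning actor's height when it meets an obstacle, running on the server only.
; It fetches front and bottom collision spheres through the ObstacleFixer interface.
; Front overlaps track filtered actors and set Z from both actors' bounds; bottom end-overlap restores the initial Z once none remain.
; On ready it also requests a navigation path to a fixed point, only printing its point count.
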(event `self.ReceiveBeginPlay`
  (bind _returnvalue (`self.GetOwner`))
  (bind (_returnvalue_x _returnvalue_y _returnvalue_z) (`KismetMathLibrary.BreakVector` (`Actor.K2_GetActorLocation` (`self.GetOwner`))))
  (if (`Actor.HasAuthority` (`self.GetOwner`))
    (if (`KismetSystemLibrary.DoesImplementInterface` (`self.GetOwner`) "/Game/Blueprints/SensitiveMesh/IObstacleFixer.IObstacleFixer_C")
      (bind _front_sphere_collision (message `/Game/Blueprints/SensitiveMesh/IObstacleFixer.Get Front Collision Sphere` _returnvalue))
      (set `self.Front Collision Sphere` _front_sphere_collision)
      (bind _bottom_collision_sphere (message `/Game/Blueprints/SensitiveMesh/IObstacleFixer.Get Bottom Collision Sphere` _returnvalue))
      (set `self.Bottom Collision Sphere` _bottom_collision_sphere)
      (set `self.Initial Z` _returnvalue_z)
      (`self.On Ready`))))

(event `On Ready`
  (add `PrimitiveComponent.OnComponentBeginOverlap` (`self.Front Collision Sphere`) (delegate `On Front Begin Overlap`))
  (bind _returnvalue (`NavigationSystem.FindPathToLocationSynchronously` (`Actor.K2_GetActorLocation` (`self.GetOwner`)) (`KismetMathLibrary.MakeVector` 0.0 0.0 180.0)))
  (`NavigationPath.EnableRecalculationOnInvalidation` _returnvalue "Enable")
  (`KismetSystemLibrary.PrintString` (`KismetStringLibrary.Conv_IntToString` (`KismetArrayLibrary.Array_Length` (`NavigationPath.PathPoints` _returnvalue))))
  (add `PrimitiveComponent.OnComponentEndOverlap` (`self.Front Collision Sphere`) (delegate `On Front End Overlap`))
  (add `PrimitiveComponent.OnComponentEndOverlap` (`self.Bottom Collision Sphere`) (delegate `On Bottom End Overlap`)))

(event `On Bottom End Overlap`
  (params (OverlappedComponent :type "PrimitiveComponent Object Reference") (OtherActor :type "Actor Object Reference") (OtherComp :type "PrimitiveComponent Object Reference") (OtherBodyIndex :type Integer))
  (if (`Actor.HasAuthority` (`self.GetOwner`))
    (if (`self.Should Overlap?` OtherActor)
      (if (== (`KismetArrayLibrary.Array_Length` (`self.Overlapping Actors`)) 0)
        (`self.Relocate` (`KismetMathLibrary.MakeVector` (.x (`Actor.K2_GetActorLocation` (`self.GetOwner`))) (.y (`Actor.K2_GetActorLocation` (`self.GetOwner`))) (`self.Initial Z`)))))))

(event `On Front End Overlap`
  (params (OverlappedComponent :type "PrimitiveComponent Object Reference") (OtherActor :type "Actor Object Reference") (OtherComp :type "PrimitiveComponent Object Reference") (OtherBodyIndex :type Integer))
  (if (`Actor.HasAuthority` (`self.GetOwner`))
    (if (`self.Should Overlap?` OtherActor)
      (`KismetArrayLibrary.Array_RemoveItem` (`self.Overlapping Actors`) OtherActor))))

(event `On Front Begin Overlap`
  (params (OverlappedComponent :type "PrimitiveComponent Object Reference") (OtherActor :type "Actor Object Reference") (OtherComp :type "PrimitiveComponent Object Reference") (OtherBodyIndex :type Integer) (bFromSweep :type Boolean) (SweepResult :type "HitResult Structure (by ref)"))
  (if (`Actor.HasAuthority` (`self.GetOwner`))
    (if (`self.Should Overlap?` OtherActor)
      (`KismetArrayLibrary.Array_Add` (`self.Overlapping Actors`) OtherActor)
      (`self.Relocate` (`self.Get Corrected Location` (`self.GetOwner`) OtherActor)))))

(event `Relocate`
  (params (`New Location` :type "Vector Structure"))
  (`Actor.K2_SetActorLocation` (`self.GetOwner`) `New Location` false false))

(fn `Get Bottom Collision Sphere`
  (returns (`Bottom Collision Sphere` :type "SphereComponent Object Reference"))
  (return null))

(fn `Get Corrected Location`
  (params (`Source Actor` :type "Actor Object Reference") (`Target Actor` :type "Actor Object Reference"))
  (returns (`Corrected Location` :type "Vector Structure"))
  (return (`KismetMathLibrary.MakeVector` (.x (`Actor.K2_GetActorLocation` (`local.Source Actor`))) (.y (`Actor.K2_GetActorLocation` (`local.Source Actor`))) (+ (.z (`.BoxExtent` (`Actor.GetActorBounds` (`local.Source Actor`) false))) (- (.z (`.BoxExtent` (`Actor.GetActorBounds` (`local.Target Actor`) false))) (.z (`Actor.K2_GetActorLocation` (`local.Source Actor`))))))))

(fn `Get Front Collision Sphere`
  (returns (`Front Sphere Collision` :type "SphereComponent Object Reference"))
  (return null))

(fn `Should Overlap?`
  (params (`Overlapped Actor` :type "Actor Object Reference"))
  (returns (ReturnValue :type Boolean))
  (return (and (!= (`local.Overlapped Actor`) (`self.GetOwner`)) (not (`Actor.ActorHasTag` (`local.Overlapped Actor`) "NotObstacle")) (!= (`GameplayStatics.GetObjectClass` (`self.GetOwner`)) (`GameplayStatics.GetObjectClass` (`local.Overlapped Actor`))))))