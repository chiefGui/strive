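; Pickup actor for a world item that shows a name widget when a main character is nearby.
; BeginPlay passes its item class to the name widget and hides it.
; Sphere overlaps toggle the widget only on the Remote (non-authority) branch, for any overlapping main character, so a listen-server host never sees it.
; A server pickup event destroys the actor; granting the item is not handled here.
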(event `self.ReceiveBeginPlay`
  (bind _asitem_name_widget (cast `/Game/Blueprints/Items/Item_Name_Widget` (`WidgetComponent.GetUserWidgetObject` (`self.Widget`))))
  (set `/Game/Blueprints/Items/Item_Name_Widget.ItemClass` (`self.Item`) _asitem_name_widget)
  (`SceneComponent.SetVisibility` (`self.Widget`) false false))

(event `self.Sphere.OnComponentBeginOverlap`
  (params (OverlappedComponent :type "PrimitiveComponent Object Reference") (OtherActor :type "Actor Object Reference") (OtherComp :type "PrimitiveComponent Object Reference") (OtherBodyIndex :type Integer) (bFromSweep :type Boolean) (SweepResult :type "HitResult Structure (by ref)"))
  (`/Engine/EditorBlueprintResources/ActorMacros.Switch Has Authority`
    (:`Remote`
      (cast `/Game/Blueprints/Characters/Main/Character_Main` OtherActor)
      (`self.Show Item Name`))))

(event `self.Sphere.OnComponentEndOverlap`
  (params (OverlappedComponent :type "PrimitiveComponent Object Reference") (OtherActor :type "Actor Object Reference") (OtherComp :type "PrimitiveComponent Object Reference") (OtherBodyIndex :type Integer))
  (`/Engine/EditorBlueprintResources/ActorMacros.Switch Has Authority`
    (:`Remote`
      (cast `/Game/Blueprints/Characters/Main/Character_Main` OtherActor)
      (`self.Hide Item Name`))))

(event `On Picked (Server)`
  (`self.K2_DestroyActor`))

(fn `Hide Item Name`
  (`SceneComponent.SetVisibility` (`self.Widget`) false false))

(fn `Show Item Name`
  (`SceneComponent.SetVisibility` (`self.Widget`) true false))

(fn `UserConstructionScript`)