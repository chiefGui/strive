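; Player state that holds a player's bag inventory, equipment slots and available skill points.
; AddItem runs on authority, filling free stacks before empty slots and recursing on overflow, with item data read from datatables via class defaults.
; AddEquipment, also authority-only, falls back to the first free slot when the requested one is taken.
; Changes to items, equipment and server-clamped skill point gains are pushed to the owning client's HUD or PlayerController.
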(event `self.ReceiveBeginPlay`
  (bind _asplayer_controller_master (cast `/Game/Blueprints/Core/PlayerControllerMaster` (`self.GetOwner`)))
  (set `self.PlayerController` _asplayer_controller_master))

(event `Refresh Inventory (Client)`
  (params (`New Slots` :type "Array of /Game/Blueprints/HUD/Inventory/Inventory_Slot_Structure Structure"))
  (`/Game/Blueprints/HUD/Master_Widget.Render Inventory` (`/Game/Blueprints/Core/PlayerControllerMaster.HUD2` (`self.PlayerController`)) `New Slots`))

(event `Increase Skill Points Available (Server)`
  (params (Amount :type Integer))
  (bind _indices (`/Game/Blueprints/Core/PlayerControllerMaster.Get Unabled Skills Indices` (`self.PlayerController`)))
  (if (not (== (`KismetArrayLibrary.Array_Length` _indices) 0))
    (bind _output_get (set `self.Skill Points Available` (`KismetMathLibrary.Clamp` (+ (`self.Skill Points Available`) Amount) 0 4)))
    (`/Game/Blueprints/Core/PlayerControllerMaster.On Skill Points Available Are Increased (Owning Client)` (`self.PlayerController`) _output_get (== _output_get 4))))

(event `Decrease Skill Points Available (Server)`
  (params (Amount :type Integer))
  (set `self.Skill Points Available` (`KismetMathLibrary.Clamp` (- (`self.Skill Points Available`) Amount) 0 4)))

(fn `Add Equipment`
  (params (Equipment :type "/Game/Blueprints/Equipments/EquipmentStrcuture Structure") (`At Index` :type Integer))
  (locals (`Decided Index To Add Equipment` :type Integer) (`New Equipments` :type "Array of /Game/Blueprints/Interactives/Items/Library/Equippables/Item_Equippable Object Reference"))
  (bind (_success_ _index) (`self.Get First Available Index At Equipments`))
  (`/Engine/EditorBlueprintResources/ActorMacros.Switch Has Authority`
    (:`Authority`
      (if (`self.Is Equipment Index Available?` (`local.At Index`))
        (set `local.Decided Index To Add Equipment` (`local.At Index`))
        (`KismetArrayLibrary.Array_Set` (`self.Equipments`) (`local.Decided Index To Add Equipment`) (`local.Equipment`) :!label _label)
        (`/Game/Blueprints/Core/PlayerControllerMaster.Refresh Equipments (Own Client)` (`self.PlayerController`) (`self.Equipments`))
        (elif _success_
          (set `local.Decided Index To Add Equipment` _index)
          (goto _label)
          (else
            ;[1 0.9403 0] TODO: Do something when equipments are full.
            (`KismetSystemLibrary.PrintString` "Equipments is full!")))))))

(fn `Add Item`
  (params (Item :type "/Game/Blueprints/Interactives/Items/Item Class Reference") (Amount :type Integer))
  (returns (`Success?` :type Boolean) (`Amount Left` :type Integer) (`Slot Index` :type Integer))
  (locals (`Slot Index To Add Item Into` :type Integer) (`Rest Amount` :type Integer))
  (bind (_sucess_ _available_slot_index) (`self.Search for the first slot available in the inventory`))
  (bind (_sucess__2 _available_slot_index_2) (`self.Search for the first slot available in the inventory`))
  (bind (_success_ _slot_index) (`self.Search for the first free stack among the slots` (`local.Item`)))
  (bind (_datatable _rowname) (break `DataTableRowHandle` (defaults `/Game/Blueprints/Core/PlayerStateMaster` (`local.Item`))))
  (bind _returnvalue (+ (`.Amount_8_B70064674ECB9A90F95B92A337BA43D0` (break `/Game/Blueprints/HUD/Inventory/Inventory_Slot_Structure` (`|GetArrayItem` (`self.Bag Items`) (`local.Slot Index To Add Item Into`)))) (`local.Amount`)))
  (`/Engine/EditorBlueprintResources/ActorMacros.Switch Has Authority`
    (:`Authority`
      (if (`self.Is Inventory Full?` Item)
        ;[0 0.04156 1] TODO: do something when inventory is completely full
        (return false 0 0)
        (else
          (bind _returnvalue_2 (`|GetDataTableRow` _datatable _rowname)
            (:`then`
              (if (`.CanBeStacked?_17_E82504DB428EE1A8DA6F8F94E703C4F0` (break `/Game/Blueprints/Interactives/Items/Item_Info_Structure` _returnvalue_2))
                (if _success_
                  (set `local.Slot Index To Add Item Into` _slot_index)
                  (if (> _returnvalue (`self.Maximum Stack Size`))
                    (set `local.Rest Amount` (- _returnvalue (`self.Maximum Stack Size`)))
                    (`KismetArrayLibrary.Array_Set` (`self.Bag Items`) (`local.Slot Index To Add Item Into`) (make `/Game/Blueprints/HUD/Inventory/Inventory_Slot_Structure` (`local.Item`) (`self.Maximum Stack Size`)))
                    (`self.Refresh Inventory (Client)` (`self.Bag Items`))
                    (bind (_success__2 _amount_left _slot_index_2) (`self.Add Item` (`local.Item`) (`local.Rest Amount`)))
                    (return true _amount_left _slot_index_2)
                    (else
                      (`KismetArrayLibrary.Array_Set` (`self.Bag Items`) (`local.Slot Index To Add Item Into`) (make `/Game/Blueprints/HUD/Inventory/Inventory_Slot_Structure` (`local.Item`) _returnvalue))
                      (`self.Refresh Inventory (Client)` (`self.Bag Items`))
                      (return true 0 (`local.Slot Index To Add Item Into`))))
                  (elif _sucess_
                    (set `local.Slot Index To Add Item Into` _available_slot_index)
                    (if (> (`local.Amount`) (`self.Maximum Stack Size`))
                      (`KismetArrayLibrary.Array_Set` (`self.Bag Items`) (`local.Slot Index To Add Item Into`) (make `/Game/Blueprints/HUD/Inventory/Inventory_Slot_Structure` (`local.Item`) (`self.Maximum Stack Size`)))
                      (`self.Refresh Inventory (Client)` (`self.Bag Items`))
                      (bind (_success__3 _amount_left_2 _slot_index_3) (`self.Add Item` (`local.Item`) (- (`local.Amount`) (`self.Maximum Stack Size`))))
                      (return true _amount_left_2 _slot_index_3)
                      (else
                        (`KismetArrayLibrary.Array_Set` (`self.Bag Items`) (`local.Slot Index To Add Item Into`) (make `/Game/Blueprints/HUD/Inventory/Inventory_Slot_Structure` (`local.Item`) (`local.Amount`)))
                        (`self.Refresh Inventory (Client)` (`self.Bag Items`))
                        (return true 0 (`local.Slot Index To Add Item Into`))))
                    (else
                      (return false (`local.Amount`) (`local.Slot Index To Add Item Into`)))))
                (elif _sucess__2
                  (bind _output_get (set `local.Slot Index To Add Item Into` _available_slot_index_2))
                  (`KismetArrayLibrary.Array_Set` (`self.Bag Items`) _output_get (make `/Game/Blueprints/HUD/Inventory/Inventory_Slot_Structure` (`local.Item`) 1))
                  (`self.Refresh Inventory (Client)` (`self.Bag Items`))
                  (if (> (`local.Amount`) 1)
                    (bind (_success__4 _amount_left_3 _slot_index_4) (`self.Add Item` (`local.Item`) (- (`local.Amount`) 1)))
                    (return true _amount_left_3 _slot_index_4)
                    (else
                      (return true 0 (`local.Slot Index To Add Item Into`))))
                  (else
                    (return false (`local.Amount`) 0)))))))))))

(fn `Get All Items`
  (returns (Items :type "Array of /Game/Blueprints/Interactives/Items/Item_Info_Structure Structure"))
  (locals (`Local Items` :type "Array of /Game/Blueprints/Interactives/Items/Item_Info_Structure Structure"))
  (for (_array_element _array_index) (`self.Equipments`)
    (if (`self.Get Equipment At Index` _array_index)
      (bind (_success_ _item_information) (`/Game/Blueprints/Helpers/Helpers.Get Item Information From Datatable` (defaults `/Game/Blueprints/Core/PlayerStateMaster` (`.ClassReference_3_2D87998A46D280BEBDE0BABDCE70B29D` (break `/Game/Blueprints/Equipments/EquipmentStrcuture` _array_element)))))
      (if _success_
        (`KismetArrayLibrary.Array_Add` (`local.Local Items`) _item_information))))
  (for (_array_element_2 _array_index_2) (`self.Bag Items`)
    (if (not (`self.Get Item Info At Slot Index` _array_index_2))
      (bind (_success__2 _item_information_2) (`/Game/Blueprints/Helpers/Helpers.Get Item Information From Datatable` (defaults `/Game/Blueprints/Core/PlayerStateMaster` (`.Item_7_B80837E54860CB76B5B5FEA55A594D88` (break `/Game/Blueprints/HUD/Inventory/Inventory_Slot_Structure` _array_element_2)))))
      (if _success__2
        (`KismetArrayLibrary.Array_Add` (`local.Local Items`) _item_information_2))))
  (return (`local.Local Items`)))

(fn `Get Amount Of Items At Index`
  (params (Index :type Integer))
  (returns (Amount :type Integer))
  (return (`.Amount_8_B70064674ECB9A90F95B92A337BA43D0` (break `/Game/Blueprints/HUD/Inventory/Inventory_Slot_Structure` (`|GetArrayItem` (`self.Bag Items`) Index)))))

(fn `Get Equipment At Index`
  (params (Index :type Integer))
  (returns (`Success?` :type Boolean) (Equipment :type "/Game/Blueprints/Equipments/EquipmentStrcuture Structure"))
  (bind _output (`|GetArrayItem` (`self.Equipments`) Index))
  (return (`KismetSystemLibrary.IsValidClass` (`.ClassReference_3_2D87998A46D280BEBDE0BABDCE70B29D` (break `/Game/Blueprints/Equipments/EquipmentStrcuture` _output))) _output))

(fn `Get Equipments By Name`
  (params (`Equipment Name` :type Name))
  (returns (`Success?` :type Boolean) (Equipments :type "Array of /Game/Blueprints/Equipments/EquipmentStrcuture Structure"))
  (locals (`Found Equipments` :type "Array of /Game/Blueprints/Equipments/EquipmentStrcuture Structure"))
  (bind _found_equipments (`local.Found Equipments`))
  (for _array_element (`self.Equipments`)
    (bind _classreference (break `/Game/Blueprints/Equipments/EquipmentStrcuture` _array_element))
    (if (`KismetSystemLibrary.IsValidClass` _classreference)
      (if (== (`.Name_2_359C4861424747F5E3870B984A1ED0E6` (break `/Game/Blueprints/Interactives/Items/Item_Info_Structure` (`.Item Information` (`/Game/Blueprints/Helpers/Helpers.Get Item Information From Datatable` (defaults `/Game/Blueprints/Core/PlayerStateMaster` _classreference))))) (`local.Equipment Name`))
        (`KismetArrayLibrary.Array_Add` (`local.Found Equipments`) _array_element))))
  (return (> (`KismetArrayLibrary.Array_Length` _found_equipments) 0) _found_equipments))

(fn `Get First Available Index At Equipments`
  (returns (`Success?` :type Boolean) (Index :type Integer))
  (locals (`Found Index` :type Integer :default -1))
  (for (_array_element _array_index) (`self.Equipments`)
    (if (not (`KismetSystemLibrary.IsValidClass` (`.ClassReference_3_2D87998A46D280BEBDE0BABDCE70B29D` (break `/Game/Blueprints/Equipments/EquipmentStrcuture` _array_element))))
      (set `local.Found Index` _array_index)
      (break)))
  (if (> (`local.Found Index`) -1)
    (return true (`local.Found Index`))
    (else
      (return false 0))))

(fn `Get Item By Name`
  (params (Name :type Name))
  (returns (Slot :type "/Game/Blueprints/HUD/Inventory/Inventory_Slot_Structure Structure") (Index :type Integer) (`Success?` :type Boolean))
  (locals (`Local Index` :type Integer) (`Local Success?` :type Boolean) (`Local Slot` :type "/Game/Blueprints/HUD/Inventory/Inventory_Slot_Structure Structure"))
  (for (_array_element _array_index) (`self.Bag Items`)
    (bind _item (break `/Game/Blueprints/HUD/Inventory/Inventory_Slot_Structure` _array_element))
    (if (`KismetSystemLibrary.IsValidClass` _item)
      (if (== (`.Name_2_359C4861424747F5E3870B984A1ED0E6` (break `/Game/Blueprints/Interactives/Items/Item_Info_Structure` (`.Item Information` (`/Game/Blueprints/Helpers/Helpers.Get Item Information From Datatable` (defaults `Object` _item))))) (`local.Name`))
        (set `local.Local Slot` _array_element)
        (set `local.Local Success?` true)
        (set `local.Local Index` _array_index)
        (break))))
  (if (`local.Local Success?`)
    (return (`local.Local Slot`) (`local.Local Index`) true)
    (else
      (return (struct) 0 false))))

(fn `Get Item Info At Slot Index`
  (params (Index :type Integer))
  (returns (`Is Slot Empty?` :type Boolean) (`Item Info` :type "/Game/Blueprints/Interactives/Items/Item_Info_Structure Structure") (Amount :type Integer))
  (bind (_item _amount) (break `/Game/Blueprints/HUD/Inventory/Inventory_Slot_Structure` (`|GetArrayItem` (`self.Bag Items`) (`local.Index`))))
  (if (`KismetSystemLibrary.IsValidClass` _item)
    (return false (`.Item Information` (`/Game/Blueprints/Helpers/Helpers.Get Item Information From Datatable` (defaults `Object` _item))) _amount)
    (else
      (return true (struct) 0))))

(fn `Is Equipment Index Available?`
  (params (Index :type Integer))
  (returns (ReturnValue :type Boolean))
  (bind _output_classreference (break `/Game/Blueprints/Equipments/EquipmentStrcuture` (`|GetArrayItem` (`self.Equipments`) Index)))
  (return (not (`KismetSystemLibrary.IsValidClass` _output_classreference))))

(fn `Is Full Of Equips?`
  (returns (`Is Full?` :type Boolean) (`Amount of Equipments` :type Integer))
  (locals (`Local Amount of Equipments` :type Integer))
  (bind _local_amount_of_equipments (`local.Local Amount of Equipments`))
  (for _array_element (`self.Equipments`)
    (if (`KismetSystemLibrary.IsValidClass` (`.ClassReference_3_2D87998A46D280BEBDE0BABDCE70B29D` (break `/Game/Blueprints/Equipments/EquipmentStrcuture` _array_element)))
      (`/Engine/EditorBlueprintResources/StandardMacros.IncrementInt` (`local.Local Amount of Equipments`))))
  (return (== _local_amount_of_equipments 6) _local_amount_of_equipments))

(fn `Is Inventory Full?`
  (params (`Item To Add` :type "/Game/Blueprints/Interactives/Items/Item Class Reference"))
  (returns (ReturnValue :type Boolean))
  (bind _returnvalue (not (`self.Search for the first slot available in the inventory`)))
  (if (`KismetSystemLibrary.IsValidClass` `Item To Add`)
    (return (and _returnvalue (not (`self.Search for the first free stack among the slots` `Item To Add`))))
    (else
      (return _returnvalue))))

(fn `Is Inventory Slot Empty?`
  (params (Index :type Integer))
  (returns (ReturnValue :type Boolean))
  (return (not (`KismetSystemLibrary.IsValidClass` (`.Item_7_B80837E54860CB76B5B5FEA55A594D88` (break `/Game/Blueprints/HUD/Inventory/Inventory_Slot_Structure` (`|GetArrayItem` (`self.Bag Items`) Index)))))))

(fn `Is Item, Equipped?`
  (params (Item :type "/Game/Blueprints/Interactives/Items/Library/Equippables/Item_Equippable Class Reference"))
  (returns (`Return Value` :type Boolean))
  (return (`self.Get Equipments By Name` (`.Name_2_359C4861424747F5E3870B984A1ED0E6` (break `/Game/Blueprints/Interactives/Items/Item_Info_Structure` (`.Item Information` (`/Game/Blueprints/Helpers/Helpers.Get Item Information From Datatable` (`.Item In Datatable` (defaults `/Game/Blueprints/Core/PlayerStateMaster` Item)))))))))

(fn `Remove Equipment At Index`
  (params (Index :type Integer))
  (`KismetArrayLibrary.Array_Set` (`self.Equipments`) Index)
  (`/Game/Blueprints/Core/PlayerControllerMaster.Refresh Equipments (Own Client)` (`self.PlayerController`) (`self.Equipments`)))

(fn `Remove Item At Index`
  (params (Index :type Integer) (Amount :type Integer))
  (returns (`Success?` :type Boolean))
  (bind _bag_items (`self.Bag Items`))
  (bind _amount (`self.Get Amount Of Items At Index` (`local.Index`)))
  (bind _output_item (break `/Game/Blueprints/HUD/Inventory/Inventory_Slot_Structure` (`|GetArrayItem` _bag_items (`local.Index`))))
  (if (and (not (`self.Is Inventory Slot Empty?` Index)) (> (`local.Amount`) 0))
    (if (> _amount (`local.Amount`))
      (`KismetArrayLibrary.Array_Set` _bag_items (`local.Index`) (make `/Game/Blueprints/HUD/Inventory/Inventory_Slot_Structure` _output_item (- _amount (`local.Amount`))))
      (`self.Refresh Inventory (Client)` (`self.Bag Items`))
      (return true)
      (else
        (`KismetArrayLibrary.Array_Set` (`self.Bag Items`) (`local.Index`) (make `/Game/Blueprints/HUD/Inventory/Inventory_Slot_Structure` null))
        (`self.Refresh Inventory (Client)` (`self.Bag Items`))
        (return true)))
    (else
      (return false))))

(fn `Search for the first free stack among the slots`
  (params (Item :type "/Game/Blueprints/Interactives/Items/Item Class Reference"))
  (returns (`Success?` :type Boolean) (`Slot Index` :type Integer))
  (locals (`Local Index` :type Integer) (`Local Bool` :type Boolean))
  (for (_array_element _array_index) (`self.Bag Items`)
    (bind (_item _amount) (break `/Game/Blueprints/HUD/Inventory/Inventory_Slot_Structure` _array_element))
    (if (`KismetSystemLibrary.IsValidClass` _item)
      (if (and (== _item Item) (< _amount (`self.Maximum Stack Size`)))
        (set `local.Local Bool` true)
        (set `local.Local Index` _array_index)
        (break))))
  (return (`local.Local Bool`) (`local.Local Index`)))

(fn `Search for the first slot available in the inventory`
  (returns (`Sucess?` :type Boolean) (`Available Slot Index` :type Integer))
  (locals (`L Is Empty?` :type Boolean) (`L Index` :type Integer))
  (for (_array_element _array_index) (`self.Bag Items`)
    (if (not (`KismetSystemLibrary.IsValidClass` (`.Item_7_B80837E54860CB76B5B5FEA55A594D88` (break `/Game/Blueprints/HUD/Inventory/Inventory_Slot_Structure` _array_element))))
      (set `local.L Is Empty?` true)
      (set `local.L Index` _array_index)
      (break)))
  (return (`local.L Is Empty?`) (`local.L Index`)))

(fn `UserConstructionScript`)