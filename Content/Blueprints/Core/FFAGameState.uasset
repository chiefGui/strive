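; FFAGameState is the game state for the free-for-all mode, tracking players and deaths on the server.
; On BeginPlay, the authority caches a reference to FFAGameMode.
; Server events register joining controllers as alive and connected, then count deaths and remove the dead from the alive list.
; The first death plays a First Blood sound on every connected player's own client.
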(event `self.ReceiveBeginPlay`
  (`/Engine/EditorBlueprintResources/ActorMacros.Switch Has Authority`
    (:`Authority`
      (bind _asffagame_mode (cast `/Game/Blueprints/Core/FFAGameMode` (`GameplayStatics.GetGameMode`)))
      (set `self.Game Mode` _asffagame_mode))))

(event `Add Player Alive (Server)`
  (params (`Player Controller` :type "/Game/Blueprints/Core/PlayerControllerMaster Object Reference"))
  (`KismetArrayLibrary.Array_Add` (`self.Players Alive`) `Player Controller`)
  (`KismetArrayLibrary.Array_Add` (`self.Players Connected`) `Player Controller`))

(event `On Player's Death (Server)`
  (params (`Dead Player Controller` :type "/Game/Blueprints/Core/PlayerControllerMaster Object Reference"))
  (`/Engine/EditorBlueprintResources/StandardMacros.IncrementInt` (`self.Number Of Deaths`)
    (:`  `
      (`KismetArrayLibrary.Array_RemoveItem` (`self.Players Alive`) `Dead Player Controller`)
      (if (== (`self.Number Of Deaths`) 1)
        (for _array_element (`self.Players Connected`)
          (`/Game/Blueprints/Core/PlayerControllerMaster.Play Sound (Own Client)` _array_element "/Game/Blueprints/SFX/Voices/FirstBlood.FirstBlood"))))))

(fn `UserConstructionScript`)