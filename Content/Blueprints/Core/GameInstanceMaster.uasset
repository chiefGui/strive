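; Game instance that owns the game's GameSparks backend session, the authenticated user and sound effect playback.
; Init creates the GameSparks and message listener objects; connection and authentication results are broadcast through event dispatchers.
; Manual and Steam logins both register the user on success, with a simulated login path using hardcoded credentials.
; It disconnects on quit or non-dedicated-server shutdown, and its sound helpers apply the stored effects volume.
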(event `self.ReceiveInit`
  (bind _returnvalue (`|GenericCreateObject` "/Script/GameSparks.GameSparksObject" self))
  (set `self.GSObject` _returnvalue)
  (bind _returnvalue_2 (`|GenericCreateObject` "/Script/GameSparks.GSMessageListenersObject" self))
  (set `self.GSListenerObject` _returnvalue_2))

(event `self.ReceiveShutdown`
  (if (not (`KismetSystemLibrary.IsDedicatedServer`))
    (`self.Disconnect User From GameSparks`)))

(event `Connect To GameSparks Request`
  (add `GameSparksObject.OnGameSparksAvailableDelegate` (`self.GSObject`) (delegate `OnGameSparksAvailable`))
  (`GameSparksObject.Connect` (`self.GSObject`) "G350631qeJ8F" "MBUoxtfWYwatG4wjAkUaCenpKFwkxq7L" true false))

(event `Before Quit`
  (`self.Disconnect User From GameSparks`))

(event `Quit`
  (`self.Before Quit`)
  (`KismetSystemLibrary.ExecuteConsoleCommand` "quit"))

(event `OnGameSparksAvailable`
  (params (available :type Boolean))
  (if available
    (`self.Connect To GameSparks Success`)))

(event `Manual User Authentication (GameSparks)`
  (params (`User Name` :type String) (Password :type String))
  (bind (_authenticationresponse _haserrors) (`GSAuthenticationRequest.SendAuthenticationRequest` Password `User Name`)
    (:`OnResponse`
      (if _haserrors
        (`self.Player Authentication Failure`)
        (else
          (`self.Handle User Authentication Success` _authenticationresponse))))))

(event `Steam User Authentication (GameSparks)`
  (params (`Session Ticket` :type String))
  (bind (_authenticationresponse _haserrors) (`GSSteamConnectRequest.SendSteamConnectRequest` false false null `Session Ticket` false true)
    (:`OnResponse`
      (if _haserrors
        (`self.Player Authentication Failure`)
        (else
          (`self.Handle User Authentication Success` _authenticationresponse))))))

(event `Simulate User Authentiaction`
  (`self.Connect To GameSparks Request`)
  (add `self.Connect To GameSparks Success` (delegate `Simulate Connect To GameSparks Success`)))

(event `Simulate Connect To GameSparks Success`
  (`self.Manual User Authentication (GameSparks)` "a" "a"))

(fn `Disconnect User From GameSparks`
  (`GameSparksObject.Disconnect` (`self.GSObject`)))

(fn `Get Sound Effects Volume`
  (returns (`Sound Effects Volume` :type "Float (double-precision)"))
  (return (`self.Sound Effects Volume`)))

(fn `Get User`
  (returns (`Player Online` :type "/Game/Core/Players/User Structure"))
  (return (`self.User`)))

(fn `Handle User Authentication Success`
  (params (`Authentication Response` :type "GSAuthenticationResponse Structure"))
  (bind ((`DisplayName` _displayname) (`UserId` _userid)) (break `GSAuthenticationResponse` `Authentication Response`))
  (`self.Register User` (make `/Game/Core/Players/User` _userid _displayname))
  (`self.Player Authentication Success` (`self.User`)))

(fn `Play Sound Effect`
  (params (`Sound Effect` :type "SoundWave Object Reference"))
  (`GameplayStatics.PlaySound2D` `Sound Effect` (`self.Get Sound Effects Volume`)))

(fn `Play Sound Effect At Location`
  (params (`Sound Effect` :type "SoundWave Object Reference") (Location :type "Vector Structure"))
  (`GameplayStatics.PlaySoundAtLocation` `Sound Effect` Location (struct) (`self.Get Sound Effects Volume`)))

(fn `Register User`
  (params (`Authenticated Player To Register` :type "/Game/Core/Players/User Structure"))
  (set `self.User` `Authenticated Player To Register`))