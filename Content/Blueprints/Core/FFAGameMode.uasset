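; Free-for-all game mode that runs a last-player-standing match.
; It registers each joining player as alive in FFAGameState and triggers their loading screen, starting once more than one is alive and ending when one remains.
; Shuffled HeroSpawn actors form a pool that GetRandomSpawn draws from without repeats.
; At Waiting Post Match it has every player's controller announce the winner; the logout check is an empty stub.
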(event `self.ReceiveBeginPlay`
  (`parent.ReceiveBeginPlay`)
  (bind _asffagame_state (cast `/Game/Blueprints/Core/FFAGameState` (`GameplayStatics.GetGameState`)))
  (set `self.Game State` _asffagame_state)
  (bind _outactors (`GameplayStatics.GetAllActorsOfClass` "/Game/Blueprints/Spawns/HeroSpawn.HeroSpawn_C"))
  (`KismetArrayLibrary.Array_Shuffle` _outactors)
  (set `self.Available Player Spawns` _outactors))

(event `self.HandleStartingNewPlayer`
  (params (NewPlayer :type "PlayerController Object Reference"))
  (bind _asplayer_controller_master (cast `/Game/Blueprints/Core/PlayerControllerMaster` NewPlayer))
  (`/Game/Blueprints/Core/FFAGameState.Add Player Alive (Server)` (`self.Game State`) _asplayer_controller_master)
  (`/Game/Blueprints/Core/PlayerControllerMaster.Append Loading Screen (Own Client)` _asplayer_controller_master))

(event `EndMatch`
  (params (NewState :type Name))
  (switch `name` NewState
    (:`WaitingPostMatch`
      (for _array_element (`GameStateBase.PlayerArray` (`self.Game State`))
        (bind _asplayer_state_master (cast `/Game/Blueprints/Core/PlayerStateMaster` _array_element))
        (`/Game/Blueprints/Core/PlayerControllerMaster.Announce Winner (Own Client)` (`/Game/Blueprints/Core/PlayerStateMaster.PlayerController` _asplayer_state_master))))))

(event `self.K2_OnLogout`
  (params (ExitingController :type "Controller Object Reference"))
  (if (== (- (`KismetArrayLibrary.Array_Length` (`GameStateBase.PlayerArray` (`self.Game State`))) 1) 0)
    _))

(fn `Get Random Spawn`
  (returns (`Random Spawn` :type "/Game/Blueprints/Spawns/HeroSpawn Object Reference"))
  (locals (`Chosen Spawn` :type "/Game/Blueprints/Spawns/HeroSpawn Object Reference"))
  (bind _output (`|GetArrayItem` (`self.Available Player Spawns`)))
  (bind _output_get (set `local.Chosen Spawn` _output))
  (`KismetArrayLibrary.Array_RemoveItem` (`self.Available Player Spawns`) _output)
  (return _output_get))

(fn `ReadyToEndMatch`
  (returns (ReturnValue :type Boolean))
  (return (or (== (`KismetArrayLibrary.Array_Length` (`/Game/Blueprints/Core/FFAGameState.Players Alive` (`self.Game State`))) 1) false)))

(fn `ReadyToStartMatch`
  (returns (ReturnValue :type Boolean))
  (bind _game_state (`self.Game State`))
  (`/Engine/EditorBlueprintResources/StandardMacros.IsValid` _game_state
    (:`Is Valid`
      (return (> (`KismetArrayLibrary.Array_Length` (`/Game/Blueprints/Core/FFAGameState.Players Alive` _game_state)) 1)))))

(fn `UserConstructionScript`)