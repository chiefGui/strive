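; Player controller for a networked click-to-move game with skills, items, equipment and multi-floor buildings.
; The server spawns the controlled character at a random Spawner and handles movement, targeting, items, skill unlocks and casts with mana and cooldown checks.
; Left click moves and targets or casts the Q-prepared skill; right-drag rotates the camera.
; Owning-client events update the HUD and building-floor visibility; RepNotifies set up HUD and view target.
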(event `self.ReceiveTick`
  (params (DeltaSeconds :type "Float (single-precision)")))

(event `On Move Character To Location (Server)`
  (params (Destination :type "Vector Structure"))
  (`/Game/Blueprints/Characters/Character_Base.Move To Location` (`self.ControlledCharacter`) Destination))

(event `Key|I`
  (params (Key :type "Key Structure"))
  (bind _hud2 (`self.HUD2`))
  ;[1 1 1] Toggle Inventory
  (:`Pressed`
    (`/Engine/EditorBlueprintResources/StandardMacros.IsValid` (`self.State`)
      (:`Is Valid`
        (`/Engine/EditorBlueprintResources/StandardMacros.FlipFlop`
          (:`A`
            (`/Game/Blueprints/HUD/Master_Widget.Show Inventory` _hud2))
          (:`B`
            (`/Game/Blueprints/HUD/Master_Widget.Hide Inventory` _hud2)))))))

(event `On Left Mouse Click`
  (bind _prepared_skill__with_state__skill (break `/Game/Blueprints/Skills/SkillWithState` (`self.Prepared Skill (With State)`)))
  (bind _state (`self.State`))
  ;[1 1 1] On Left Mouse Click
  (`/Engine/EditorBlueprintResources/StandardMacros.IsValid` _state
    (:`Is Valid`
      (if (`/Game/Levels/FreeForAll/Master_PlayerState.Is Dead?` _state)
        _
        (elif (`KismetSystemLibrary.IsValidClass` _prepared_skill__with_state__skill)
          (bind (_location _hitactor) (`self.Get Click Information`))
          (`self.Cast Skill (Server)` (`self.Prepared Skill (With State)`) _location _hitactor)
          (set `self.Prepared Skill (With State)` (struct))
          (else
            (bind (_location_2 _hitactor_2) (`self.Get Click Information`))
            (`self.On Set Current Target (Server)` _hitactor_2)
            (`self.On Move Character To Location (Server)` _location_2)))))))

(event `Key|RightMouseButton`
  (params (Key :type "Key Structure"))
  ;[1 1 1] Unprepare skill
  (:`Pressed`
    (set `self.Prepared Skill (With State)` (struct))))

(event `Key|Q`
  (params (Key :type "Key Structure"))
  ;[1 1 1] Prepare skill to cast when pressed Q
  (:`Pressed`
    (`self.Prepare skill to cast (Not Replicated)` (`|GetArrayItem` (`/Game/Blueprints/Characters/Main/Character_Main.Skills` (`self.ControlledCharacter`))))))

(event `On Set Current Target (Server)`
  (params (`New Current Target` :type "Actor Object Reference"))
  ;[1 1 1] Set Current Target (Server)
  (`/Engine/EditorBlueprintResources/StandardMacros.IsValid` `New Current Target`
    (:`Is Valid`
      (set `/Game/Blueprints/Characters/Character_Base.CurrentTarget` `New Current Target` (`self.ControlledCharacter`)))))

(event `InputAction|SetDestination`
  (params (Key :type "Key Structure"))
  ;[1 1 1] Handle Left Mouse Click
  (:`Pressed`
    (`/Engine/EditorBlueprintResources/StandardMacros.DoOnce` false :!label _label
      (:`Completed`
        (`|ExecutionSequence`
          (:`then_0`
            (goto _label_2 :!via `Open`))
          (:`then_1`
            (`/Engine/EditorBlueprintResources/StandardMacros.Gate` true :!label _label_2
              (:`Exit`
                (`|ExecutionSequence`
                  (:`then_0`
                    (`self.On Left Mouse Click`))
                  (:`then_1`
                    (`KismetSystemLibrary.Delay` 0.2)
                    (goto _label_2))))))))))
  (:`Released`
    (`|ExecutionSequence`
      (:`then_0`
        (goto _label_2 :!via `Close`))
      (:`then_1`
        (`KismetSystemLibrary.Delay` 0.2)
        (goto _label :!via `Reset`)))))

(event `On Skill Points Available Are Increased (Owning Client)`
  (params (`New Amount Of Skill Points Available` :type Integer) (`Reached Max Allowed?` :type Boolean))
  (`/Game/Blueprints/HUD/Master_Widget.Show Upgrade Skill Buttons` (`self.HUD2`)))

(event `On Consume Item (Server)`
  (params (Item :type "/Game/Blueprints/Items/Library/Consumables/Item_Consumable Class Reference") (`Index At Inventory` :type Integer))
  (`|ExecutionSequence`
    (:`then_0`
      (`/Game/Levels/FreeForAll/Master_PlayerState.Remove Item At Index` (`self.State`) `Index At Inventory` 1))
    (:`then_1`
      (`|SpawnActorFromClass` Item (`KismetMathLibrary.MakeTransform` (0.0 0.0 0.0) (struct) (0.0 0.0 0.0)) "Undefined" "OverrideRootScale" self (`self.ControlledCharacter`) self null))))

(event `Enable Skill At Index (Server)`
  (params (Index :type Integer))
  (bind (_new_skill_with_state _success_) (`self.Enable Skill At Index` Index))
  (if _success_
    (`self.On Skill Is Enabled (Owning Client)` Index _new_skill_with_state (`/Game/Levels/FreeForAll/Master_PlayerState.Skill Points Available` (`self.State`)))
    (bind _aspassive_skill (castclass `/Game/Blueprints/Skills/Library/Passive/PassiveSkill` (`.Skill_3_01C3ED4C4A86F0F2FC12D09B6FAEBC11` (break `/Game/Blueprints/Skills/SkillWithState` _new_skill_with_state))))
    (`self.Activate Passive Skill (Server)` _aspassive_skill)))

(event `Prepare skill to cast (Not Replicated)`
  (params (Skill :type "/Game/Blueprints/Skills/SkillWithState Structure"))
  (bind (_skill _isincooldown_ _isenabled_) (break `/Game/Blueprints/Skills/SkillWithState` Skill))
  ;[1 1 1] Prepare skill to cast
  (castclass `/Game/Blueprints/Skills/Library/Active/ActiveSkill` _skill)
  (if _isenabled_
    (set `self.Prepared Skill (With State)` Skill)))

(event `Cast Skill (Server)`
  (params (`Skill With State` :type "/Game/Blueprints/Skills/SkillWithState Structure") (`Final Location` :type "Vector Structure") (`Final Actor` :type "Actor Object Reference"))
  ;[1 1 1] Cast Skill
  (`self.Resolve Skill Cast (On Server)` `Skill With State` `Final Location` `Final Actor`))

(event `On Skill Is Enabled (Owning Client)`
  (params (`Skill Index` :type Integer) (`New Skill With State` :type "/Game/Blueprints/Skills/SkillWithState Structure") (`Skill Points Available Remaining` :type Integer))
  (`/Game/Blueprints/HUD/Master_Widget.Update Skill State At Index` (`self.HUD2`) `New Skill With State` `Skill Index`)
  (if (> `Skill Points Available Remaining` 0)
    (`/Game/Blueprints/HUD/Master_Widget.Hide Upgrade Skill Button At Index` (`self.HUD2`) `Skill Index`)
    (else
      (`/Game/Blueprints/HUD/Master_Widget.Hide All Upgrade Skill Buttons` (`self.HUD2`)))))

(event `On Unequip Item (Server)`
  (params (Item :type "/Game/Blueprints/Items/Library/Equippables/Item_Equippable Class Reference") (`Index at Equipments` :type Integer))
  (bind _state (`self.State`))
  (`|ExecutionSequence`
    (:`then_0`
      (`/Game/Levels/FreeForAll/Master_PlayerState.Add Item` _state Item 1))
    (:`then_1`
      (`/Game/Levels/FreeForAll/Master_PlayerState.Remove Equipment At Index` _state `Index at Equipments`))))

(event `On Equip Item (Server)`
  (params (Item :type "/Game/Blueprints/Items/Library/Equippables/Item_Equippable Class Reference") (`Index At Inventory` :type Integer) (`Index At Equipments` :type Integer))
  (`|ExecutionSequence`
    (:`then_0`
      (`/Game/Levels/FreeForAll/Master_PlayerState.Remove Item At Index` (`self.State`) `Index At Inventory` 1))
    (:`then_1`
      (bind _returnvalue (`|SpawnActorFromClass` Item (`KismetMathLibrary.MakeTransform` (0.0 0.0 0.0) (struct) (0.0 0.0 0.0)) "Undefined" "OverrideRootScale" self (`self.ControlledCharacter`) self null))
      (`/Game/Levels/FreeForAll/Master_PlayerState.Add Equipment (Server)` (`self.State`) _returnvalue `Index At Equipments`))))

(event `Start Skill Cooldown (Server)`
  (params (`Skill With State` :type "/Game/Blueprints/Skills/SkillWithState Structure"))
  (bind (_skill _isincooldown_) (break `/Game/Blueprints/Skills/SkillWithState` `Skill With State`))
  (bind (_metadata_name _metadata_description _metadata_icon _metadata_manacost _metadata_casttime _metadata_cooldowntime) (break `/Game/Blueprints/Skills/SkillMetadata` (defaults `/Game/Blueprints/Core/MainPlayerController` _skill)))
  ;[1 1 1] Start Cooldown of Casted Skill
  (if _isincooldown_
    (`self.On Skill State Has Changed (Owning Client)` `Skill With State`)
    (`KismetSystemLibrary.Delay` _metadata_cooldowntime)
    (bind _new_skill_with_state (`self.Set Cooldown For Skill` _skill))
    (`self.On Skill State Has Changed (Owning Client)` _new_skill_with_state)))

(event `On Unequip Item (Own Client)`
  (params (`At Equipments Index` :type Integer))
  (`/Game/Blueprints/HUD/Master_Widget.Remove Equipment At Index` (`self.HUD2`) `At Equipments Index`))

(event `InputAxisKey|MouseX`
  (params (AxisValue :type "Float (single-precision)"))
  ;[1 1 1] Camera rotation
  (`self.Rotate Camera` AxisValue))

(event `Activate Passive Skill (Server)`
  (params (`Passive Skill` :type "/Game/Blueprints/Skills/Library/Passive/PassiveSkill Class Reference"))
  (`|SpawnActorFromClass` `Passive Skill` (`KismetMathLibrary.MakeTransform` (0.0 0.0 0.0) (struct) (0.0 0.0 0.0)) "Undefined" "OverrideRootScale" self null))

(event `Key|RightMouseButton`
  (params (Key :type "Key Structure"))
  ;[1 1 1] Camera rotation
  (:`Pressed`
    (set `self.IsRMBPressed` true))
  (:`Released`
    (set `self.IsRMBPressed` false)))

(event `On Skill State Has Changed (Owning Client)`
  (params (`New Skill With State` :type "/Game/Blueprints/Skills/SkillWithState Structure"))
  (bind (_skill_with_state _index _success_) (`self.Get Skill With State` (`.Skill_3_01C3ED4C4A86F0F2FC12D09B6FAEBC11` (break `/Game/Blueprints/Skills/SkillWithState` `New Skill With State`))))
  ;[1 1 1] When Skill Cooldown Has Changed
  (if _success_
    (`/Game/Blueprints/HUD/Master_Widget.Update Skill State At Index` (`self.HUD2`) `New Skill With State` _index)))

(event `On Equip Item (Own Client)`
  (params (`Added Equipment` :type "/Game/Blueprints/Items/Library/Equippables/Item_Equippable Class Reference") (Index :type Integer) (Equipments :type "Array of /Game/Blueprints/Items/Library/Equippables/Item_Equippable Object Reference"))
  (`KismetSystemLibrary.PrintString` (`KismetSystemLibrary.GetDisplayName` (`|GetArrayItem` Equipments))))

(event `On Cast Skill (Client)`
  (params (`Mana Lost` :type Integer) (`New Current Mana` :type Integer)))

(event `On Character Enter Building's Floor (Own Client)`
  (params (Building :type "/Game/Levels/ABuilding Object Reference") (`Floor Index` :type Integer))
  (`/Game/Levels/ABuilding.Show Floor By Index` Building `Floor Index`)
  (`/Game/Levels/ABuilding.Hide Floors Above` Building `Floor Index`)
  (`/Game/Levels/ABuilding.Show Actors At Floor` Building `Floor Index`)
  (`/Game/Levels/ABuilding.Hide Actors Outside Floor` Building `Floor Index`))

(event `On Another Character Enter Building's Floor (Own Client)`
  (params (`Self Floor` :type Integer) (Character :type "/Game/Blueprints/Characters/Character_Base Object Reference") (Building :type "/Game/Levels/ABuilding Object Reference"))
  (`/Game/Levels/ABuilding.Show Actors At Floor` Building `Self Floor`)
  (`/Game/Levels/ABuilding.Hide Actors Outside Floor` Building `Self Floor`))

(event `Update HP HUD`
  (params (`New Current HP` :type Integer))
  (`/Game/Blueprints/HUD/Master_Widget.Update HP` (`self.HUD2`) `New Current HP`))

(event `Update Mana HUD`
  (params (`New Current Mana` :type Integer))
  (`/Game/Blueprints/HUD/Master_Widget.Update Mana` (`self.HUD2`) `New Current Mana`))

(event `On Actor Is Spawned Inside Building's Floor (Own Client)`
  (params (Actor :type "Actor Object Reference") (Building :type "/Game/Levels/ABuilding Object Reference"))
  (`KismetSystemLibrary.PrintString` (`KismetStringLibrary.Conv_BoolToString` (`/Game/Levels/ABuilding.Is Actor Inside Building?` Building (`self.ControlledCharacter`)))))

(event `self.ReceiveBeginPlay`
  ;[1 1 1] BeginPlay
  (`/Engine/EditorBlueprintResources/ActorMacros.Switch Has Authority`
    (:`Authority`
      (bind _asmaster_player_state (cast `/Game/Levels/FreeForAll/Master_PlayerState` (`self.PlayerState`)))
      (set `self.State` _asmaster_player_state)
      (bind _outactors (`GameplayStatics.GetAllActorsOfClass` "/Game/Levels/FreeForAll/Spawner.Spawner_C"))
      (bind (_returnvalue_location _returnvalue_rotation) (`KismetMathLibrary.BreakTransform` (`self.GetTransform` (`|GetArrayItem` _outactors (`KismetMathLibrary.RandomInteger` (- (`KismetArrayLibrary.Array_Length` _outactors) 1))))))
      (bind _returnvalue (`|SpawnActorFromClass` "/Game/Blueprints/Characters/Main/Character_Main.Character_Main_C" (`KismetMathLibrary.MakeTransform` _returnvalue_location _returnvalue_rotation) "Undefined" "OverrideRootScale" self (`self.State`) null))
      (set `self.ControlledCharacter` _returnvalue)
      (`/Game/Blueprints/Helpers/Time_Macros.Repeater` 0.1
        (:`On Every Interval`
          (if (not (`/Game/Levels/FreeForAll/Master_PlayerState.Is Dead?` (`self.State`)))
            (`/Game/Blueprints/Characters/Character_Base.While Alive` (`self.ControlledCharacter`))))))
    (:`Remote`
      (set `self.bShowMouseCursor` true))))

(fn `Can Cast Skill?`
  (params (`Skill With State` :type "/Game/Blueprints/Skills/SkillWithState Structure"))
  (returns (`Insufficient Mana?` :type Boolean) (`In Cooldown?` :type Boolean) (`Unabled?` :type Boolean) (`Success?` :type Boolean))
  (bind (_metadata_name _metadata_description _metadata_icon _metadata_manacost) (break `/Game/Blueprints/Skills/SkillMetadata` (defaults `/Game/Blueprints/Core/MainPlayerController` (`.Skill_3_01C3ED4C4A86F0F2FC12D09B6FAEBC11` (break `/Game/Blueprints/Skills/SkillWithState` (`local.Skill With State`))))))
  (`/Engine/EditorBlueprintResources/ActorMacros.Switch Has Authority`
    (:`Authority`
      (if (`.IsEnabled?_8_D7AF8FBB449B5BC509A7FDAAA0FBA04D` (break `/Game/Blueprints/Skills/SkillWithState` `Skill With State`))
        (if (`.IsInCooldown?_6_E0C35E734066415EDBC9BB81DAACD8C6` (break `/Game/Blueprints/Skills/SkillWithState` (`local.Skill With State`)))
          (return true true false false)
          (elif (>= (`/Game/Levels/FreeForAll/Master_PlayerState.Current Mana` (`self.State`)) _metadata_manacost)
            (return false false false true)
            (else
              (return true false false false))))
        (else
          (return false false true false))))))

(fn `Enable Skill At Index`
  (params (Index :type Integer))
  (returns (`New Skill With State` :type "/Game/Blueprints/Skills/SkillWithState Structure") (`Success?` :type Boolean))
  (bind (_output_skill _output_isincooldown_) (break `/Game/Blueprints/Skills/SkillWithState` (`|GetArrayItem` (`/Game/Blueprints/Characters/Main/Character_Main.Skills` (`self.ControlledCharacter`)) Index)))
  (bind _skillwithstate (make `/Game/Blueprints/Skills/SkillWithState` _output_skill _output_isincooldown_ true))
  (if (`KismetSystemLibrary.IsValidClass` _output_skill)
    (`KismetArrayLibrary.Array_Set` (`/Game/Blueprints/Characters/Main/Character_Main.Skills` (`self.ControlledCharacter`)) (`local.Index`) _skillwithstate)
    (`/Game/Levels/FreeForAll/Master_PlayerState.Decrease Skill Points Available (Server)` (`self.State`) 1)
    (return _skillwithstate true)
    (else
      (return (struct) false))))

(fn `Get Click Information`
  (returns (Location :type "Vector Structure") (HitActor :type "Actor Object Reference") (`IsNavigable?` :type Boolean))
  (bind (_bblockinghit _binitialoverlap _time _distance _location _impactpoint _normal _impactnormal _physmat _hitactor) (`GameplayStatics.BreakHitResult` (`self.GetHitResultUnderCursorByChannel` "TraceTypeQuery1")))
  (return _location _hitactor _bblockinghit))

(fn `Get Skill With State`
  (params (Skill :type "/Game/Blueprints/Skills/Skill Class Reference"))
  (returns (`Skill With State` :type "/Game/Blueprints/Skills/SkillWithState Structure") (Index :type Integer) (`Success?` :type Boolean))
  (locals (`Found?` :type Boolean) (`Index Found` :type Integer) (`Skill With State Found` :type "/Game/Blueprints/Skills/SkillWithState Structure"))
  (bind _metadata_name (break `/Game/Blueprints/Skills/SkillMetadata` (defaults `/Game/Levels/FreeForAll/Master_PlayerState` (`local.Skill`))))
  (for (_array_element _array_index) (`/Game/Blueprints/Characters/Main/Character_Main.Skills` (`self.ControlledCharacter`))
    (bind _metadata_name_2 (break `/Game/Blueprints/Skills/SkillMetadata` (defaults `/Game/Levels/FreeForAll/Master_PlayerState` (`.Skill_3_01C3ED4C4A86F0F2FC12D09B6FAEBC11` (break `/Game/Blueprints/Skills/SkillWithState` _array_element)))))
    (if (== _metadata_name_2 _metadata_name)
      (set `local.Found?` true)
      (set `local.Index Found` _array_index)
      (set `local.Skill With State Found` _array_element)
      (break)))
  (return (`local.Skill With State Found`) (`local.Index Found`) (`local.Found?`)))

(fn `Get Unabled Skills Indices`
  (returns (Indices :type "Array of Integer") (`Can Ultimate Be Enabled?` :type Boolean))
  (locals (`Unabled Skills Indices` :type "Array of Integer"))
  (bind _unabled_skills_indices (`local.Unabled Skills Indices`))
  (for (_array_element _array_index) (`/Game/Blueprints/Characters/Main/Character_Main.Skills` (`self.ControlledCharacter`))
    (if (not (`.IsEnabled?_8_D7AF8FBB449B5BC509A7FDAAA0FBA04D` (break `/Game/Blueprints/Skills/SkillWithState` _array_element)))
      (`KismetArrayLibrary.Array_Add` (`local.Unabled Skills Indices`) _array_index)))
  (return _unabled_skills_indices (== (`KismetArrayLibrary.Array_LastIndex` _unabled_skills_indices) 0)))

(fn `OnRep_ControlledCharacter`
  (bind _state (`self.State`))
  (bind _controlledcharacter (`self.ControlledCharacter`))
  (`self.SetViewTargetWithBlend` (`self.ControlledCharacter`))
  (`/Engine/EditorBlueprintResources/ActorMacros.Switch Has Authority`
    (:`Authority`
      (bind _output_get (set `/Game/Levels/FreeForAll/Master_PlayerState.Max HP` (`/Game/Blueprints/Characters/Character_Base.MaxHP` _controlledcharacter) _state))
      (set `/Game/Levels/FreeForAll/Master_PlayerState.Current HP` _output_get _state)
      (bind _output_get_2 (set `/Game/Levels/FreeForAll/Master_PlayerState.Max Mana` (`/Game/Blueprints/Characters/Character_Base.MaxMana` _controlledcharacter) _state))
      (set `/Game/Levels/FreeForAll/Master_PlayerState.Current Mana` _output_get_2 _state))))

(fn `OnRep_State`
  (`/Engine/EditorBlueprintResources/ActorMacros.Switch Has Authority`
    (:`Remote`
      (bind _returnvalue (`|CreateWidget` "/Game/Blueprints/HUD/Master_Widget.Master_Widget_C" null (`self.ControlledCharacter`) self (`self.State`)))
      (bind _output_get (set `self.HUD2` _returnvalue))
      (`UserWidget.AddToViewport` _output_get 0))))

(fn `Render Custom Cursor`
  (bind _returnvalue (`|CreateWidget` "/Game/Blueprints/Cursors/Cursor.Cursor_C"))
  (`UserWidget.AddToViewport` _returnvalue 0)
  (set `self.MouseCursorWidgetRef` _returnvalue))

(fn `Resolve Skill Cast (On Server)`
  (params (`Skill With State` :type "/Game/Blueprints/Skills/SkillWithState Structure") (`Final Location` :type "Vector Structure") (`Final Actor` :type "Actor Object Reference"))
  (bind _skill_with_state_skill (break `/Game/Blueprints/Skills/SkillWithState` (`local.Skill With State`)))
  (`/Engine/EditorBlueprintResources/ActorMacros.Switch Has Authority`
    (:`Authority`
      (if (`.Success?` (`self.Can Cast Skill?` (`local.Skill With State`)))
        (`/Game/Blueprints/Characters/Main/Character_Main.On Cast Skill (Multicast)` (`self.ControlledCharacter`))
        (bind _asactive_skill (castclass `/Game/Blueprints/Skills/Library/Active/ActiveSkill` _skill_with_state_skill))
        (`|SpawnActorFromClass` _asactive_skill (`KismetMathLibrary.MakeTransform` (0.0 0.0 0.0)) "Undefined" "OverrideRootScale" self (`local.Final Location`) (`local.Final Actor`) null)
        (bind _new_skill_with_state (`self.Set Cooldown For Skill` _asactive_skill true))
        (`self.Start Skill Cooldown (Server)` _new_skill_with_state)
        (bind (_metadata_name _metadata_description _metadata_icon _metadata_manacost) (break `/Game/Blueprints/Skills/SkillMetadata` (defaults `/Game/Blueprints/Core/MainPlayerController` _asactive_skill)))
        (bind _new_current_mana (`/Game/Levels/FreeForAll/Master_PlayerState.Decrease Mana` (`self.State`) _metadata_manacost))
        (`self.On Cast Skill (Client)` _metadata_manacost _new_current_mana)
        (else
          (set `self.Prepared Skill (With State)` (struct)))))))

(fn `Rotate Camera`
  (params (Axis :type "Float (double-precision)"))
  (locals (RotationRate :type "Float (double-precision)"))
  (if (< Axis 0.0)
    (set `local.RotationRate` -2.0)
    (else
      (set `local.RotationRate` 1.0)))
  (if (`self.IsRMBPressed`)
    (`SceneComponent.K2_AddWorldRotation` (`/Game/Blueprints/Characters/Main/Character_Main.SpringArm` (`self.ControlledCharacter`)) (`KismetMathLibrary.MakeRotator` 0.0 0.0 (+ Axis (`local.RotationRate`))) false false)))

(fn `Set Cooldown For Skill`
  (params (Skill :type "/Game/Blueprints/Skills/Skill Class Reference") (`In Cooldown?` :type Boolean))
  (returns (`New Skill With State` :type "/Game/Blueprints/Skills/SkillWithState Structure"))
  (bind (_skill_with_state _index _success_) (`self.Get Skill With State` Skill))
  (bind (_skill _isincooldown_ _isenabled_) (break `/Game/Blueprints/Skills/SkillWithState` _skill_with_state))
  (bind _skillwithstate (make `/Game/Blueprints/Skills/SkillWithState` _skill (`local.In Cooldown?`) _isenabled_))
  (if _success_
    (`KismetArrayLibrary.Array_Set` (`/Game/Blueprints/Characters/Main/Character_Main.Skills` (`self.ControlledCharacter`)) _index _skillwithstate)
    (return _skillwithstate)))

(fn `UserConstructionScript`)

(fn `Validate Range With Actors`)