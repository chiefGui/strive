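; Bush actor that conceals actors standing inside it by hiding them and disabling their clickability.
; The server tracks occupants through collision box overlaps, ignoring an enter that repeats the last added actor.
; Multicasts apply hiding on remote machines only and restore the leaving actor.
; The server also notifies ABaseCharacter occupants of each enter or leave, passing the bush, and notifies a leaving character of its own exit.
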(event `Hide Actor (Server)`
  (params (Actor :type "Actor Object Reference"))
  (`self.SetActorHiddenInGame` Actor true)
  (`/Game/Blueprints/Helpers/Helpers.Toggle Actor Clickability` Actor))

(event `self.Collision Box.OnComponentBeginOverlap`
  (params (OverlappedComponent :type "PrimitiveComponent Object Reference") (OtherActor :type "Actor Object Reference") (OtherComp :type "PrimitiveComponent Object Reference") (OtherBodyIndex :type Integer) (bFromSweep :type Boolean) (SweepResult :type "HitResult Structure (by ref)"))
  (`/Engine/EditorBlueprintResources/ActorMacros.Switch Has Authority`
    (:`Authority`
      (if (not (`self.Is Actor Same As Last One?` OtherActor))
        (`KismetArrayLibrary.Array_Add` (`self.Actors Inside`) OtherActor)
        (`self.On Actor Enter Bush (Multicast)` OtherActor (`self.Actors Inside`))
        (for _array_element (`self.Actors Inside`)
          (bind _asabase_character (cast `/Game/Blueprints/Characters/ABaseCharacter` _array_element))
          (`/Game/Blueprints/Characters/ABaseCharacter.On Actor Enter Bush (Server)` _asabase_character OtherActor self))))))

(event `On Actor Enter Bush (Multicast)`
  (params (`Actor That Entered` :type "Actor Object Reference") (`Actors Inside` :type "Array of Actor Object Reference"))
  (`/Engine/EditorBlueprintResources/ActorMacros.Switch Has Authority`
    (:`Remote`
      (for _array_element `Actors Inside`
        (`/Engine/EditorBlueprintResources/StandardMacros.IsValid` _array_element
          (:`Is Valid`
            (`self.SetActorHiddenInGame` _array_element true)
            (`/Game/Blueprints/Helpers/Helpers.Toggle Actor Clickability` _array_element)))))))

(event `self.Collision Box.OnComponentEndOverlap`
  (params (OverlappedComponent :type "PrimitiveComponent Object Reference") (OtherActor :type "Actor Object Reference") (OtherComp :type "PrimitiveComponent Object Reference") (OtherBodyIndex :type Integer))
  (`/Engine/EditorBlueprintResources/ActorMacros.Switch Has Authority`
    (:`Authority`
      (`self.On Actor Leave Bush (Multicast)` OtherActor (`self.Actors Inside`))
      (`KismetArrayLibrary.Array_RemoveItem` (`self.Actors Inside`) OtherActor)
      (for _array_element (`self.Actors Inside`)
        (bind _asabase_character (cast `/Game/Blueprints/Characters/ABaseCharacter` _array_element))
        (`/Game/Blueprints/Characters/ABaseCharacter.On Actor Leave Bush (Server)` _asabase_character OtherActor self))
      (bind _asabase_character_2 (cast `/Game/Blueprints/Characters/ABaseCharacter` OtherActor))
      (`/Game/Blueprints/Characters/ABaseCharacter.On Actor Leave Bush (Server)` _asabase_character_2 _asabase_character_2 self))))

(event `On Actor Leave Bush (Multicast)`
  (params (`Actor That Left` :type "Actor Object Reference") (`Actors Inside` :type "Array of Actor Object Reference"))
  (`/Engine/EditorBlueprintResources/ActorMacros.Switch Has Authority`
    (:`Remote`
      (`self.SetActorHiddenInGame` `Actor That Left` false)
      (`/Game/Blueprints/Helpers/Helpers.Toggle Actor Clickability` `Actor That Left` true))))

(fn `Is Actor Same As Last One?`
  (params (Actor :type "Actor Object Reference"))
  (returns (`Return Value` :type Boolean))
  (bind _actors_inside (`self.Actors Inside`))
  (if (> (`KismetArrayLibrary.Array_Length` _actors_inside) 0)
    (return (== Actor (`|GetArrayItem` _actors_inside (`KismetArrayLibrary.Array_LastIndex` _actors_inside))))
    (else
      (return false))))

(fn `UserConstructionScript`)